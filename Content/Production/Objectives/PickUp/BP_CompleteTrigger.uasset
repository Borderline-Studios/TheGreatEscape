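; Trigger actor for pickup objectives that holds the train until the objective is complete.
; When a TrainEngine overlaps its Box, it stores the engine and calls ToggleTrainStop on it.
; Tick polls ObjectiveComplete, which this graph never sets, and toggles the stored engine again through a DoOnce once the flag is true.
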(event `self.ReceiveBeginPlay`)

(event `self.ReceiveTick`
  (params (DeltaSeconds :type "Float (single-precision)"))
  (bind _as_train_engine (`self.As Train Engine`))
  (if (`self.ObjectiveComplete`)
    (if (`KismetSystemLibrary.IsValid` _as_train_engine)
      (`/Engine/EditorBlueprintResources/StandardMacros.DoOnce` false
        (:`Completed`
          (`TrainEngine.ToggleTrainStop` _as_train_engine))))))

(event `self.Box.OnComponentBeginOverlap`
  (params (OverlappedComponent :type "PrimitiveComponent Object Reference") (OtherActor :type "Actor Object Reference") (OtherComp :type "PrimitiveComponent Object Reference") (OtherBodyIndex :type Integer) (bFromSweep :type Boolean) (SweepResult :type "HitResult Structure (by ref)"))
  (bind _astrain_engine (cast `TrainEngine` OtherActor))
  (bind _output_get (set `self.As Train Engine` _astrain_engine))
  (`TrainEngine.ToggleTrainStop` _output_get))

(fn `UserConstructionScript`)