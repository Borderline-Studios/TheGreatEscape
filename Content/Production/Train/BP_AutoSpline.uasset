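; Track actor that merges the train engine's track splines into one continuous spline at runtime.
; BeginPlay finds BP_TrainEngine; a one-shot Tick step, delayed half a second, fetches its spline references.
; It copies world-space point locations in array order, skipping each segment's last point except the final one, without copying tangents or rotations.
; It then passes itself to the engine through BPOverrideTrack.
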(event `self.ReceiveBeginPlay`
  (bind _returnvalue (`GameplayStatics.GetActorOfClass` "/Game/Production/Train/BP_TrainEngine.BP_TrainEngine_C"))
  (bind _output_get (set `self.TrainRef` _returnvalue))
  (if (`KismetSystemLibrary.IsValid` _output_get)
    _))

(event `self.ReceiveTick`
  (params (DeltaSeconds :type "Float (single-precision)"))
  (bind _spline (`self.Spline`))
  (bind _spline_2 (`self.Spline`))
  (bind _spline_references (`self.Spline References`))
  (bind _spline_3 (`self.Spline`))
  (bind _returnvalue (`SplineTrack.GetSplineComponent` (`|GetArrayItem` (`self.Spline References`))))
  (bind _returnvalue_2 (`KismetMathLibrary.Conv_IntToDouble` (`SplineComponent.GetNumberOfSplinePoints` (`self.Spline`))))
  (bind _returnvalue_3 (`SplineTrack.GetSplineComponent` (`|GetArrayItem` _spline_references (`KismetArrayLibrary.Array_LastIndex` _spline_references))))
  (bind _returnvalue_4 (- (`KismetMathLibrary.FTrunc` _returnvalue_2) 1))
  (`KismetSystemLibrary.Delay` 0.5)
  (`/Engine/EditorBlueprintResources/StandardMacros.DoOnce` false
    (:`Completed`
      (`|ExecutionSequence`
        (:`then_0`
          (if (`KismetSystemLibrary.IsValid` (`self.TrainRef`))
            (bind _array (`TrainEngine.GetSplineReferences` (`self.TrainRef`)))
            (set `self.Spline References` _array)))
        (:`then_1`
          (`SplineComponent.SetLocationAtSplinePoint` _spline_2 0 (`SplineComponent.GetLocationAtSplinePoint` _returnvalue 0 "World") "World" true)
          (`SplineComponent.SetLocationAtSplinePoint` _spline_2 1 (`SplineComponent.GetLocationAtSplinePoint` _returnvalue 1 "World") "World" true)
          (for (_array_element _array_index) _spline_references
            (if (== _array_index 0)
              (bind _returnvalue_5 (`SplineTrack.GetSplineComponent` _array_element))
              (bind _returnvalue_6 (- (`SplineComponent.GetNumberOfSplinePoints` _returnvalue_5) 2))
              (for _index (range 2 (+ _returnvalue_6 1))
                (`SplineComponent.AddPoint` (`self.Spline`) (make `SplinePoint` _returnvalue_2) true)
                (`SplineComponent.SetLocationAtSplinePoint` _spline _returnvalue_4 (`SplineComponent.GetLocationAtSplinePoint` _returnvalue_5 _index (`self.Coordinate Space`)) "World" true)
                (`SplineComponent.SetLocationAtSplinePoint` (`self.Spline`) _returnvalue_4 (`SplineComponent.GetLocationAtSplinePoint` _returnvalue_5 _index (`self.Coordinate Space`)) "World" true))
              (else
                (for _index_2 (range (+ _returnvalue_6 1))
                  (`SplineComponent.AddPoint` _spline (make `SplinePoint` _returnvalue_2) true)
                  (`SplineComponent.SetLocationAtSplinePoint` _spline _returnvalue_4 (`SplineComponent.GetLocationAtSplinePoint` _returnvalue_5 _index_2 (`self.Coordinate Space`)) "World" true)))))
          (`SplineComponent.AddPoint` _spline_3 (make `SplinePoint` _returnvalue_2) true)
          (`SplineComponent.SetLocationAtSplinePoint` _spline_3 _returnvalue_4 (`SplineComponent.GetLocationAtSplinePoint` _returnvalue_3 (- (`SplineComponent.GetNumberOfSplinePoints` _returnvalue_3) 1) (`self.Coordinate Space`)) "World" true))
        (:`then_2`
          (`TrainEngine.BPOverrideTrack` (`self.TrainRef`) self))))))

(fn `UserConstructionScript`)