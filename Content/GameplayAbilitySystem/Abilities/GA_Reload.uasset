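; Gameplay ability that reloads the first-person player's gun and refills its ammo to a fixed amount.
; On activation it flags the player character as reloading, then swaps the gun's skeletal mesh to the reload version and plays its animation.
; A fixed delay, rather than an animation callback, times the refill and return to the idle mesh and animation.
; The ability then ends and clears the reloading flag.
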(event `self.K2_ActivateAbility`
  (bind _asbp_first_person_character (cast `/Game/FirstPerson/Blueprints/BP_FirstPersonCharacter` (`GameplayStatics.GetPlayerPawn` 0))
    (:`then`
      (set `/Game/FirstPerson/Blueprints/BP_FirstPersonCharacter.IsReloading` true _asbp_first_person_character)
      (bind _gun (`/Game/FirstPerson/Blueprints/BP_FirstPersonCharacter.Gun` _asbp_first_person_character))
      (`SkinnedMeshComponent.SetSkinnedAssetAndUpdate` _gun "/Game/VericalSlice/Characters/Player/Animation/Reload/A_Player_Reload.A_Player_Reload" true)
      (`SkeletalMeshComponent.PlayAnimation` _gun "/Game/VericalSlice/Characters/Player/Animation/Reload/A_Player_Reload_Anim.A_Player_Reload_Anim" false)
      (`KismetSystemLibrary.Delay` 3.0)
      (set `/Game/FirstPerson/Blueprints/BP_FirstPersonCharacter.Ammo` 6 _asbp_first_person_character)
      (`SkinnedMeshComponent.SetSkinnedAssetAndUpdate` _gun "/Game/VericalSlice/Characters/Player/Animation/Idle/A_Player_Idle.A_Player_Idle" true)
      (`SkeletalMeshComponent.PlayAnimation` _gun "/Game/VericalSlice/Characters/Player/Animation/Idle/A_Player_Idle_Anim.A_Player_Idle_Anim" false))
    (:`CastFailed`
      _))
  (`self.K2_EndAbility`)
  (set `/Game/FirstPerson/Blueprints/BP_FirstPersonCharacter.IsReloading` false _asbp_first_person_character))