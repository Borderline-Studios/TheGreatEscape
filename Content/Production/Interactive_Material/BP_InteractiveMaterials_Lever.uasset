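; Interactive lever that the player rotates by holding left or right mouse while aiming at it, driving material progress on linked actors and meshes.
; A looping timer line-traces from screen center against the lever mesh and flags hover through custom primitive data.
; While hovered, input moves AnimProgress at constant speed, lerps the rotation, and pushes the value through SetMaterialProgress or custom primitive data.
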(event `self.ReceiveBeginPlay`
  (set `self.RotationMin` (`SceneComponent.RelativeRotation` (`self.StaticMeshComponent`)))
  (set `self.RotationMax` (`KismetMathLibrary.ComposeRotators` (`self.RotationMin`) (struct :`Pitch` 55.0)))
  (`self.SetCurrentRotation` (`self.AnimProgress`))
  (bind _returnvalue (`KismetSystemLibrary.K2_SetTimerDelegate` (delegate `UpdateMaterials`) (`self.MaterialsUpdateFreq`) true))
  (set `self.MaterialsUpdateTimer` _returnvalue))

(event `UpdateMaterials`
  (bind _returnvalue (`GameplayStatics.GetPlayerController` 0))
  (bind _returnvalue_2 (`KismetSystemLibrary.K2_GetTimerElapsedTimeHandle` (`self.MaterialsUpdateTimer`)))
  (bind _ishovered (`self.IsHoveredByCursor`))
  (`PrimitiveComponent.SetCustomPrimitiveDataFloat` (`self.StaticMeshComponent`) 0 (`KismetMathLibrary.SelectFloat` 1.0 0.0 _ishovered))
  (if _ishovered
    (`|ExecutionSequence`
      (:`then_0`
        (if (`PlayerController.IsInputKeyDown` _returnvalue "LeftMouseButton")
          (set `self.AnimProgress` (`KismetMathLibrary.FInterpTo_Constant` (`self.AnimProgress`) 1.0 _returnvalue_2 (`self.RotationSpeed`)))
          (`self.SetCurrentRotation` (`self.AnimProgress`) :!label _label)))
      (:`then_1`
        (if (`PlayerController.IsInputKeyDown` _returnvalue "RightMouseButton")
          (set `self.AnimProgress` (`KismetMathLibrary.FInterpTo_Constant` (`self.AnimProgress`) 0.0 _returnvalue_2 (`self.RotationSpeed`)))
          (goto _label)))
      (:`then_2`
        (for _array_element (`self.ActorsToControl`)
          (`/Game/Production/Interactive_Material/BP_InteractiveMaterials_ControllableMesh.SetMaterialProgress` _array_element (`self.AnimProgress`))))
      (:`then_3`
        (for _array_element_2 (`self.MeshesToControl`)
          (`PrimitiveComponent.SetCustomPrimitiveDataFloat` (`StaticMeshActor.StaticMeshComponent` _array_element_2) 0 (`self.AnimProgress`)))))))

(fn `IsHoveredByCursor`
  (returns (IsHovered :type Boolean))
  (bind _returnvalue (`WidgetLayoutLibrary.GetPlayerScreenWidgetGeometry` (`GameplayStatics.GetPlayerController` 0)))
  (bind (_returnvalue_x _returnvalue_y) (`KismetMathLibrary.BreakVector2D` (`SlateBlueprintLibrary.GetAbsoluteSize` _returnvalue)))
  (bind (_worldlocation _worlddirection) (`PlayerController.DeprojectScreenPositionToWorld` (`GameplayStatics.GetPlayerController` 0) (/ _returnvalue_x 2.0) (/ _returnvalue_y 2.0)))
  (bind (_hitlocation _hitnormal _bonename _outhit _returnvalue_2) (`PrimitiveComponent.K2_LineTraceComponent` (`self.StaticMeshComponent`) _worldlocation (+ _worldlocation (* _worlddirection (`self.HoverDistanceFromPlayerMax`))) false false false))
  (return _returnvalue_2))

(fn `SetCurrentRotation`
  (params (Progress :type "Float (double-precision)"))
  (`SceneComponent.K2_SetRelativeRotation` (`self.StaticMeshComponent`) (`KismetMathLibrary.RLerp` (`self.RotationMin`) (`self.RotationMax`) Progress true) false false))

(fn `UserConstructionScript`)