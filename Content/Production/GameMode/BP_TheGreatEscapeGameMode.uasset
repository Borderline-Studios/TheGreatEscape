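; Game mode for The Great Escape that runs round-based enemy waves, with music and sound cues.
; When CheckNumOfEnemyLeft finds no enemies alive, it calls CallRespawnEnemy for the next wave or advances the round, adding a wave per round.
; Round changes update the player's round, swap music by round number and pause between fades and stingers.
; Clearing the final round hides gameplay UI, fades out and shows the end-game widget.
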(event `self.ReceiveBeginPlay`
  (bind _asbp_first_person_character (cast `/Game/Production/BackUp/BP_FirstPersonCharacter` (`GameplayStatics.GetPlayerPawn` 0)))
  (set `self.PlayerRef` _asbp_first_person_character)
  (`GameplayStatics.PlaySoundAtLocation` "/Game/Production/SoundEffects/SFX_snare.SFX_snare" (0.0 0.0 0.0) (struct) 1.0 1.0 0.0 null null null null)
  (`KismetSystemLibrary.Delay` 1.8)
  (`AudioComponent.FadeIn` (`self.Audio`) 10.0 1.0 0.0 "Linear"))

(event `CheckNumOfEnemyLeft`
  (bind _returnvalue (`GameplayStatics.GetPlayerController` 0))
  (bind _numofenemiesalive (`self.NumOfEnemiesAlive`))
  (bind _audio (`self.Audio`))
  (bind _wavenumber (`self.WaveNumber`))
  (bind _roundnumber (`self.RoundNumber`))
  (bind _returnvalue_2 (`self.K2_GetActorLocation` (`self.PlayerRef`)))
  ;[1 1 1] Check how many enemies are left, if 0 spawn more
  (`KismetSystemLibrary.PrintString` (`KismetStringLibrary.Conv_IntToString` _numofenemiesalive))
  (if (== _numofenemiesalive 0)
    (if (== _wavenumber (`self.MaxWavesPerRound`))
      (if (== (`self.RoundNumber`) (`self.MaxRounds`))
        ;[1 0 0] ADD WIN CONDITION FROM TRUE
        (`Widget.SetVisibility` (`/Game/Production/BackUp/BP_FirstPersonCharacter.GameplayUI` (`self.PlayerRef`)) "Hidden")
        (`PlayerCameraManager.StartCameraFade` :`self` (`GameplayStatics.GetPlayerCameraManager` 0) :`ToAlpha` 1.0 :`Duration` 5.0 :`bShouldFadeAudio` true :`bHoldWhenFinished` true)
        (bind _returnvalue_3 (`|CreateWidget` "/Game/Production/UI/Blueprints/WBP_EndGameUI.WBP_EndGameUI_C" _returnvalue))
        (`UserWidget.AddToViewport` _returnvalue_3 0)
        (`WidgetBlueprintLibrary.SetInputMode_UIOnlyEx` _returnvalue _returnvalue_3)
        (else
          (if (== (`self.RoundNumber`) (- (`self.MaxRounds`) 1))
            (`AudioComponent.SetSound` _audio "/Game/Production/SoundEffects/Music/M_DrumsOfWar.M_DrumsOfWar")
            (else
              (`AudioComponent.SetSound` _audio "/Game/Production/SoundEffects/Music/M_amb_Guitar.M_amb_Guitar")))
          (`/Engine/EditorBlueprintResources/StandardMacros.IncrementInt` (`self.MaxWavesPerRound`)
            (:`  `
              (`/Engine/EditorBlueprintResources/StandardMacros.IncrementInt` _roundnumber
                (:`  `
                  (set `self.WaveNumber` 1)
                  (set `/Game/Production/BackUp/BP_FirstPersonCharacter.CurrentRound` _roundnumber (`self.PlayerRef`))
                  (`AudioComponent.FadeOut` (`self.Audio`) 2.0 0.0 "Linear")
                  (`KismetSystemLibrary.Delay` 1.3)
                  (`GameplayStatics.PlaySoundAtLocation` "/Game/Production/SoundEffects/SFX_GuitarSting.SFX_GuitarSting" _returnvalue_2 (struct) 1.0 1.0 0.0 null null null null)
                  (`KismetSystemLibrary.Delay` (`self.RoundDelay`))
                  (`GameplayStatics.PlaySoundAtLocation` "/Game/Production/SoundEffects/SFX_snare.SFX_snare" _returnvalue_2 (struct) 1.0 1.0 0.0 null null null null)
                  (`self.RespawnEnemy` true)
                  (`AudioComponent.FadeIn` (`self.Audio`) 10.0 1.0 0.0 "Linear")))))))
      (else
        (`/Engine/EditorBlueprintResources/StandardMacros.IncrementInt` (`self.WaveNumber`)
          (:`  `
            (`KismetSystemLibrary.PrintString` (`KismetStringLibrary.Concat_StrStr` "Wave Number:" (`KismetStringLibrary.Conv_IntToString` _wavenumber)))
            (`self.RespawnEnemy` false)))))))

(fn `UserConstructionScript`)