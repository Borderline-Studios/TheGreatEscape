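; BP_TriggerDoor is a one-shot door that moves when a specific referenced actor leaves its detection component.
; On BeginPlay it caches the mesh start position and a target marker position, and derives the timeline play rate from the movement time, taken from the door sound's duration when valid.
; The end-overlap event passes a DoOnce, plays the sound and runs a timeline that lerps the mesh to the target without sweeping.
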(event `self.ReceiveBeginPlay`
  (bind _doorsound (`self.DoorSound`))
  (set `self.StartPos` (`SceneComponent.K2_GetComponentLocation` (`self.StaticMesh`)))
  (set `self.EndPos` (`SceneComponent.K2_GetComponentLocation` (`self.PositionToMoveTo`)))
  (if (`KismetSystemLibrary.IsValid` _doorsound)
    (set `self.TimeToCompleteMovement` (`SoundBase.Duration` _doorsound)))
  (`TimelineComponent.SetPlayRate` (`self.Timeline_0`) (/ 1.0 (`self.TimeToCompleteMovement`))))

(event `self.DetectionComponent.OnComponentEndOverlap`
  (params (OverlappedComponent :type "PrimitiveComponent Object Reference") (OtherActor :type "Actor Object Reference") (OtherComp :type "PrimitiveComponent Object Reference") (OtherBodyIndex :type Integer))
  (if (== OtherActor (`self.ActorReference`))
    (`/Engine/EditorBlueprintResources/StandardMacros.DoOnce` false
      (:`Completed`
        (`GameplayStatics.PlaySoundAtLocation` (`self.DoorSound`) (`self.K2_GetActorLocation`) (struct) 1.0 1.0 0.0 null null null null)
        (bind (_direction _lerpalpha) (`Timeline|Timeline_0` :!via `PlayFromStart`)
          (:`Update`
            (`SceneComponent.K2_SetWorldLocation` (`self.StaticMesh`) (`KismetMathLibrary.VLerp` (`self.StartPos`) (`self.EndPos`) _lerpalpha) false false)))))))

(fn `UserConstructionScript`)