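; BP_LED is an environment LED text display that feeds a configurable string through a 2D scene capture.
; The construction script restricts the capture to the TextRender component and applies the Text variable to it.
; It then shifts the text along local X in steps based on its rendered width, leaving Y and Z untouched.
; The event graph holds no active logic.
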(fn `UserConstructionScript`
  (bind _textrender (`self.TextRender`))
  (bind (_returnvalue_x _returnvalue_y) (`KismetMathLibrary.BreakVector` (`TextRenderComponent.GetTextLocalSize` _textrender)))
  (bind (_relativelocation_x _relativelocation_y _relativelocation_z) (`KismetMathLibrary.BreakVector` (`SceneComponent.RelativeLocation` _textrender)))
  (`SceneCaptureComponent.ShowOnlyComponent` (`self.SceneCaptureComponent2D`) (`self.TextRender`))
  (`TextRenderComponent.K2_SetText` (`self.TextRender`) (`self.Text`))
  (`SceneComponent.K2_SetRelativeLocation` _textrender (`KismetMathLibrary.MakeVector` (`KismetMathLibrary.Conv_IntToDouble` (* (`KismetMathLibrary.FFloor` (/ _returnvalue_y 15.0)) 10)) _relativelocation_y _relativelocation_z) false false))