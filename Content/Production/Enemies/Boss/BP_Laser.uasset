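; BP_Laser is a boss laser hazard that damages the player character when it touches the laser mesh.
; On BeginPlay it caches the player and their ability system component.
; Begin overlap applies the GE_LaserDamage gameplay effect through that component and calls the player's PostHitProcess, so damage is triggered once per overlap entry.
; End overlap clears a PlayerBeingHit flag, which nothing in this graph sets or reads.
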(event `self.ReceiveBeginPlay`
  (bind _asbp_player_character (cast `/Game/Production/Player/Character/BP_PlayerCharacter` (`GameplayStatics.GetPlayerCharacter` 0)))
  (bind _output_get (set `self.PlayerRef` _asbp_player_character))
  (set `self.GameplayAbilityComp` (`AbilitySystemBlueprintLibrary.GetAbilitySystemComponent` _output_get)))

(event `self.LaserMesh.OnComponentBeginOverlap`
  (params (OverlappedComponent :type "PrimitiveComponent Object Reference") (OtherActor :type "Actor Object Reference") (OtherComp :type "PrimitiveComponent Object Reference") (OtherBodyIndex :type Integer) (bFromSweep :type Boolean) (SweepResult :type "HitResult Structure (by ref)"))
  (cast `/Game/Production/Player/Character/BP_PlayerCharacter` OtherActor)
  (if (`KismetSystemLibrary.IsValid` (`self.GameplayAbilityComp`))
    (`AbilitySystemComponent.BP_ApplyGameplayEffectToSelf` :`self` (`self.GameplayAbilityComp`) :`GameplayEffectClass` "/Game/Production/GameplayAbilitySystem/Effeects/GE_LaserDamage.GE_LaserDamage_C" :`Level` 1.0)
    (`PlayerCharacter.PostHitProcess` (`self.PlayerRef`))))

(event `self.LaserMesh.OnComponentEndOverlap`
  (params (OverlappedComponent :type "PrimitiveComponent Object Reference") (OtherActor :type "Actor Object Reference") (OtherComp :type "PrimitiveComponent Object Reference") (OtherBodyIndex :type Integer))
  (cast `/Game/Production/Player/Character/BP_PlayerCharacter` OtherActor)
  (set `self.PlayerBeingHit` false))

(fn `UserConstructionScript`)