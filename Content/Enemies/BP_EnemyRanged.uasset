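; BP_EnemyRanged is a ranged enemy character that reports its spawn and death to BP_TheGreatEscapeGameMode's live-enemy count.
; BeginPlay applies default stats through a Gameplay Ability System effect and increments that count.
; Tick polls a gameplay attribute, presumably health, and triggers a one-time ragdoll at zero or below.
; Ragdoll sets a short lifespan and, after an equal delay, decrements the count and requests a remaining-enemy check.
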(event `self.ReceiveBeginPlay`
  ;[1 1 1] When spawned in, increase amount of enemies alive
  (`AbilitySystemComponent.BP_ApplyGameplayEffectToSelf` :`self` (`self.AbilitySystemComponent`) :`GameplayEffectClass` "/Game/GameplayAbilitySystem/Effects/GE_EnemyDefaults.GE_EnemyDefaults_C")
  (bind _asbp_the_great_escape_game_mode (cast `/Game/VericalSlice/Core/GameModes/BP_TheGreatEscapeGameMode` (`GameplayStatics.GetGameMode`))
    (:`then`
      (`/Engine/EditorBlueprintResources/StandardMacros.IncrementInt` (`/Game/VericalSlice/Core/GameModes/BP_TheGreatEscapeGameMode.NumOfEnemiesAlive` _asbp_the_great_escape_game_mode)))
    (:`CastFailed`
      (`KismetSystemLibrary.PrintString` "game mdoe cast fail begin play ranged"))))

(event `self.ReceiveTick`
  (params (DeltaSeconds :type "Float (single-precision)"))
  (if (<= (`.ReturnValue` (`AbilitySystemComponent.GetGameplayAttributeValue` (`self.AbilitySystemComponent`) (struct :`AttributeName` "Health" :`Attribute` "/Script/TheGreatEscape.GASAttributeSet:Health" :`AttributeOwner` "Class'\"/Script/TheGreatEscape.GASAttributeSet\"'"))) 0.0)
    (if (not (`self.bDying`))
      (set `self.bDying` true)
      (`KismetSystemLibrary.PrintString` "dead ranged enemy")
      (`self.Ragdoll`))))

(event `Ragdoll`
  ;[1 1 1] Ragdoll - do physics object stuff on character
  (`PrimitiveComponent.SetSimulatePhysics` (`self.Mesh`) true)
  (`CharacterMovementComponent.DisableMovement` (`self.CharacterMovement`))
  (`self.SetLifeSpan` self 3.0)
  (`KismetSystemLibrary.Delay` 3.0)
  (bind _asbp_the_great_escape_game_mode (cast `/Game/VericalSlice/Core/GameModes/BP_TheGreatEscapeGameMode` (`GameplayStatics.GetGameMode`))
    (:`then`
      (`/Engine/EditorBlueprintResources/StandardMacros.DecrementInt` (`/Game/VericalSlice/Core/GameModes/BP_TheGreatEscapeGameMode.NumOfEnemiesAlive` _asbp_the_great_escape_game_mode)
        (:`  `
          (`/Game/VericalSlice/Core/GameModes/BP_TheGreatEscapeGameMode.CheckNumOfEnemyLeft` _asbp_the_great_escape_game_mode))))
    (:`CastFailed`
      (`KismetSystemLibrary.PrintString` "failed game mode"))))

(fn `UserConstructionScript`)