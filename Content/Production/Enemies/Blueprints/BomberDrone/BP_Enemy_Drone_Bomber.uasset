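; Bomber drone enemy that homes in on the player and detonates on contact.
; DetectionSphere overlap sets the player's first-person camera as the ProjectileMovement homing target.
; ExplodeSphere overlap triggers a short delay, then explosion VFX and sound at the player's captured location, and the drone destroys itself.
; The blast applies a GAS effect through the player's own ability system, runs the player's post-hit processing and shakes the camera.
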(event `self.Explode`
  (params (Location :type "Vector Structure"))
  (bind _as_player_character (`self.As Player Character`))
  (bind _returnvalue (`AbilitySystemBlueprintLibrary.GetAbilitySystemComponent` _as_player_character))
  (`KismetSystemLibrary.Delay` 0.3)
  (`NiagaraFunctionLibrary.SpawnSystemAtLocation` "/Game/Production/Effects/Enemies/Hit_Kill/NS_Explosion.NS_Explosion" Location)
  (`GameplayStatics.PlaySoundAtLocation` "/Game/Production/Enemies/Blueprints/BomberDrone/Bomber_ExplodeSFX.Bomber_ExplodeSFX" Location (struct) 1.0 1.0 0.0 null null null null)
  (`AbilitySystemComponent.BP_ApplyGameplayEffectToTarget` :`self` _returnvalue :`GameplayEffectClass` "/Game/Production/BackUp/GameplayAbilitySystem/Effects/GE_BomberDroneEffect.GE_BomberDroneEffect_C" :`Target` _returnvalue :`Level` 1.0)
  (`PlayerCharacter.PostHitProcess` _as_player_character)
  (`PlayerCameraManager.StartCameraShake` :`self` (`GameplayStatics.GetPlayerCameraManager` 0) :`ShakeClass` "/Game/Production/Player/Character/CameraEffects/ExplosionCamShake.ExplosionCamShake_C" :`Scale` 4.0)
  (`self.K2_DestroyActor`))

(event `self.TargetPlayer`
  (bind _projectilemovementcomponent (`self.ProjectileMovementComponent`))
  (bind _asbp_player_character (cast `/Game/Production/Player/Character/BP_PlayerCharacter` (`GameplayStatics.GetPlayerPawn` 0)))
  (set `ProjectileMovementComponent.HomingTargetComponent` (`PlayerCharacter.FirstPersonCameraComponent` _asbp_player_character) _projectilemovementcomponent)
  (set `ProjectileMovementComponent.InitialSpeed` (`MovementComponent.GetMaxSpeed` _projectilemovementcomponent) _projectilemovementcomponent))

(event `self.ReceiveBeginPlay`
  (bind _asplayer_character (cast `PlayerCharacter` (`GameplayStatics.GetPlayerPawn` 0)))
  (set `self.As Player Character` _asplayer_character))

(event `self.DetectionSphere.OnComponentBeginOverlap`
  (params (OverlappedComponent :type "PrimitiveComponent Object Reference") (OtherActor :type "Actor Object Reference") (OtherComp :type "PrimitiveComponent Object Reference") (OtherBodyIndex :type Integer) (bFromSweep :type Boolean) (SweepResult :type "HitResult Structure (by ref)"))
  (cast `PlayerCharacter` OtherActor)
  (`self.TargetPlayer`))

(event `self.ExplodeSphere.OnComponentBeginOverlap`
  (params (OverlappedComponent :type "PrimitiveComponent Object Reference") (OtherActor :type "Actor Object Reference") (OtherComp :type "PrimitiveComponent Object Reference") (OtherBodyIndex :type Integer) (bFromSweep :type Boolean) (SweepResult :type "HitResult Structure (by ref)"))
  (bind _as_player_character (`self.As Player Character`))
  (if (== OtherActor _as_player_character)
    (`self.Explode` (`self.K2_GetActorLocation` _as_player_character))))

(fn `UserConstructionScript`)