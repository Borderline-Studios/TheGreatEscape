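; DeadLock gameplay ability that spends the player's whole magazine on one delayed, piercing hitscan shot.
; It aborts during melee, reload or empty ammo; otherwise it multi-traces from the camera view and applies GE_Damage to every hit with an ability system component.
; Components tagged Headshot award extra score and feedback.
; It then auto-reloads and delays ending the ability for several seconds after firing.
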(event `self.K2_ActivateAbility`
  (bind _returnvalue (`GameplayStatics.GetPlayerPawn` 0))
  (bind (_location _rotation) (`Controller.GetPlayerViewPoint` (`GameplayStatics.GetPlayerController` 0)))
  (bind _asbp_first_person_character (cast `/Game/Production/BackUp/BP_FirstPersonCharacter` (`GameplayStatics.GetPlayerPawn` 0))
    (:`then`
      (if (or (`/Game/Production/BackUp/BP_FirstPersonCharacter.IsMelee` _asbp_first_person_character) (`/Game/Production/BackUp/BP_FirstPersonCharacter.IsReloading` _asbp_first_person_character))
        (`self.K2_EndAbility` :!label _label)
        (set `/Game/Production/BackUp/BP_FirstPersonCharacter.IsShooting` false _asbp_first_person_character)
        (else
          (set `/Game/Production/BackUp/BP_FirstPersonCharacter.IsShooting` true _asbp_first_person_character)
          (if (> (`/Game/Production/BackUp/BP_FirstPersonCharacter.Ammo` _asbp_first_person_character) 0)
            (set `/Game/Production/BackUp/BP_FirstPersonCharacter.Ammo` 0 _asbp_first_person_character)
            (`GameplayStatics.PlaySoundAtLocation` "/Game/VericalSlice/SoundEffects/SFX_Gunshot.SFX_Gunshot" (0.0 0.0 0.0) (struct) 0.1 (* 0.7 (`GameplayStatics.GetGlobalTimeDilation`)) 0.0 null null null null)
            (`KismetSystemLibrary.Delay` 0.2)
            (`SkeletalMeshComponent.PlayAnimation` (`/Game/Production/BackUp/BP_FirstPersonCharacter.SkeletalMesh_Gun` _asbp_first_person_character) "/Game/VericalSlice/Characters/Player/Animation/Fire/A_Player_Fire_Anim.A_Player_Fire_Anim" false)
            (bind _outhits (`KismetSystemLibrary.LineTraceMulti` _location (+ _location (* _rotation 18000.0)) "TraceTypeQuery2" false (`|MakeArray` _asbp_first_person_character :!type "Actor Object Reference") "None" true (struct :`R` 0.226841 :`G` 1.0 :`A` 1.0) (struct :`R` 1.0 :`B` 0.079394 :`A` 1.0)))
            (for _array_element _outhits
              (bind (_bblockinghit _binitialoverlap _time _distance _location_2 _impactpoint _normal _impactnormal _physmat _hitactor _hitcomponent) (`GameplayStatics.BreakHitResult` _array_element))
              (bind _returnvalue_2 (`AbilitySystemBlueprintLibrary.GetAbilitySystemComponent` _hitactor))
              (`/Engine/EditorBlueprintResources/StandardMacros.IsValid` _returnvalue_2
                (:`Is Valid`
                  (if (`ActorComponent.ComponentHasTag` _hitcomponent "Headshot")
                    (bind _asbp_first_person_character_2 (cast `/Game/Production/BackUp/BP_FirstPersonCharacter` _returnvalue))
                    (set `/Game/Production/BackUp/BP_FirstPersonCharacter.HitEnemy` true _asbp_first_person_character_2)
                    (set `/Game/Production/BackUp/BP_FirstPersonCharacter.HeadShot` true _asbp_first_person_character_2)
                    (set `/Game/Production/BackUp/BP_FirstPersonCharacter.Score` (+ (`/Game/Production/BackUp/BP_FirstPersonCharacter.Score` _asbp_first_person_character_2) 20) _asbp_first_person_character_2)
                    (`GameplayStatics.PlaySoundAtLocation` "/Game/VericalSlice/SoundEffects/SFX_Hit_01_Cue.SFX_Hit_01_Cue" (0.0 0.0 0.0) (struct) 0.1 1.5 0.0 null null null null)
                    (else
                      (bind _asbp_first_person_character_3 (cast `/Game/Production/BackUp/BP_FirstPersonCharacter` _returnvalue))
                      (set `/Game/Production/BackUp/BP_FirstPersonCharacter.HitEnemy` true _asbp_first_person_character_3)
                      (set `/Game/Production/BackUp/BP_FirstPersonCharacter.Score` (+ (`/Game/Production/BackUp/BP_FirstPersonCharacter.Score` _asbp_first_person_character_3) 10) _asbp_first_person_character_2)))
                  (`AbilitySystemComponent.BP_ApplyGameplayEffectToSelf` :`self` _returnvalue_2 :`GameplayEffectClass` "/Game/Production/BackUp/GameplayAbilitySystem/Effects/GE_Damage.GE_Damage_C" :`Level` 1.0)
                  (`GameplayStatics.PlaySoundAtLocation` "/Game/VericalSlice/SoundEffects/SFX_Hit_01.SFX_Hit_01" (0.0 0.0 0.0) (struct) 1.0 1.0 0.0 null null null null))))
            (`KismetSystemLibrary.Delay` 0.3)
            (if (<= (`/Game/Production/BackUp/BP_FirstPersonCharacter.Ammo` _asbp_first_person_character) 0)
              (`/Game/Production/BackUp/BP_FirstPersonCharacter.AutoReload` _asbp_first_person_character))
            (set `/Game/Production/BackUp/BP_FirstPersonCharacter.IsShooting` false _asbp_first_person_character)
            (`KismetSystemLibrary.Delay` 5.0)
            (`self.K2_EndAbility`)
            (else
              (goto _label))))))
    (:`CastFailed`
      (`KismetSystemLibrary.Delay` 5.0)
      (`self.K2_EndAbility`))))