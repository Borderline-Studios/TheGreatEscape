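; Zipline actor that carries the player from a start post to an end post when they overlap its trigger box.
; At BeginPlay it builds a two-point spline between the posts and removes the trigger unless the start is higher.
; On overlap, timelines snap the player to the nearest spline point, temporarily made the spline's start, then move them to the end.
; Ladder-named variables drive this; the DisableInput call is disconnected.
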(event `self.ReceiveBeginPlay`
  (bind (_returnvalue_x _returnvalue_y _returnvalue_z) (`KismetMathLibrary.BreakVector` (`SceneComponent.K2_GetComponentLocation` (`self.EndPost`))))
  (bind (_returnvalue_x_2 _returnvalue_y_2 _returnvalue_z_2) (`KismetMathLibrary.BreakVector` (`SceneComponent.K2_GetComponentLocation` (`self.StartPost`))))
  (bind _returnvalue (`GameplayStatics.GetActorOfClass` "/Game/Production/Player/Character/BP_PlayerCharacter.BP_PlayerCharacter_C"))
  (set `self.PlayerRef` _returnvalue)
  (`self.SplineSetup`)
  (`TimelineComponent.SetPlayRate` (`self.CenterPlayerOnLadder`) (`self.PlayerSnapMultiplier`))
  (`TimelineComponent.SetPlayRate` (`self.PlayerAscendLadder`) (`self.TraversalSpeedMultiplier`))
  (if (<= _returnvalue_z_2 _returnvalue_z)
    (`ActorComponent.K2_DestroyComponent` (`self.Box`))))

(event `self.Box.OnComponentBeginOverlap`
  (params (OverlappedComponent :type "PrimitiveComponent Object Reference") (OtherActor :type "Actor Object Reference") (OtherComp :type "PrimitiveComponent Object Reference") (OtherBodyIndex :type Integer) (bFromSweep :type Boolean) (SweepResult :type "HitResult Structure (by ref)"))
  (bind _playerref (`self.PlayerRef`))
  (bind _playermovespline (`self.PlayerMoveSpline`))
  (bind _returnvalue (`self.K2_GetActorLocation` _playerref))
  (bind _returnvalue_2 (`SplineComponent.FindLocationClosestToWorldLocation` (`self.PlayerMoveSpline`) _returnvalue "World"))
  (if (and (== OtherActor _playerref) (not (`self.bPlayerClimbingLadder`)))
    (set `self.bPlayerClimbingLadder` true)
    (set `self.PlayerLerpStart` _returnvalue)
    (set `self.PlayerLerpEnd` _returnvalue_2)
    (`SplineComponent.SetLocationAtSplinePoint` (`self.PlayerMoveSpline`) 0 _returnvalue_2 "World" true)
    (bind (_direction _playerlerptospline) (`Timeline|CenterPlayerOnLadder` :!via `PlayFromStart`)
      (:`Update`
        (`self.K2_SetActorLocation` (`self.PlayerRef`) (`KismetMathLibrary.VLerp` (`self.PlayerLerpStart`) (`self.PlayerLerpEnd`) _playerlerptospline) false false))
      (:`Finished`
        (bind (_direction_2 _playerascendalpha) (`Timeline|PlayerAscendLadder` :!via `PlayFromStart`)
          (:`Update`
            (`self.K2_SetActorLocation` (`self.PlayerRef`) (`SplineComponent.GetLocationAtDistanceAlongSpline` _playermovespline (`KismetMathLibrary.Lerp` 0.0 (`SplineComponent.GetSplineLength` _playermovespline) _playerascendalpha) "World") false false))
          (:`Finished`
            (`self.EnableInput` (`self.PlayerRef`) null)
            (`SplineComponent.SetLocationAtSplinePoint` (`self.PlayerMoveSpline`) 0 (`self.SplineStart`) "World" true)
            (set `self.bPlayerClimbingLadder` false)))))))

(fn `DisableCollision`
  (`PrimitiveComponent.SetCollisionEnabled` (`self.Box`) "NoCollision"))

(fn `EnableCollision`
  (`PrimitiveComponent.SetCollisionEnabled` (`self.Box`) "QueryOnly"))

(fn `SplineSetup`
  (bind _playermovespline (`self.PlayerMoveSpline`))
  (bind _returnvalue (`SceneComponent.K2_GetComponentLocation` (`self.StartPost`)))
  (`SplineComponent.SetLocationAtSplinePoint` _playermovespline 0 _returnvalue "World" true)
  (set `self.SplineStart` _returnvalue)
  (`SplineComponent.SetLocationAtSplinePoint` _playermovespline 1 (`SceneComponent.K2_GetComponentLocation` (`self.EndPost`)) "World" true)
  (`SplineComponent.SetTangentAtSplinePoint` _playermovespline 0 (0.0 0.0 0.0) "World" true)
  (`SplineComponent.SetTangentAtSplinePoint` _playermovespline 1 (0.0 0.0 0.0) "World" true)
  (return))

(fn `UserConstructionScript`)