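; Gameplay ability for a DeadLock gunshot that spends the first-person character's entire remaining ammo, ending immediately if reloading or empty.
; After the sound and a short delay, it plays the fire animation and runs a debug-drawn multi line trace from the view point.
; Hits with an Ability System Component set hit flags, with extra headshot feedback by component tag.
; GE_Damage targets both victim and shooter, using the non-headshot branch's character cast.
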(event `self.K2_ActivateAbility`
  (bind _returnvalue (`GameplayStatics.GetPlayerPawn` 0))
  (bind (_location _rotation) (`Controller.GetPlayerViewPoint` (`GameplayStatics.GetPlayerController` 0)))
  (bind _asbp_first_person_character (cast `/Game/FirstPerson/Blueprints/BP_FirstPersonCharacter` (`GameplayStatics.GetPlayerPawn` 0))
    (:`then`
      (if (`/Game/FirstPerson/Blueprints/BP_FirstPersonCharacter.IsReloading` _asbp_first_person_character)
        (`self.K2_EndAbility` :!label _label)
        (elif (> (`/Game/FirstPerson/Blueprints/BP_FirstPersonCharacter.Ammo` _asbp_first_person_character) 0)
          (set `/Game/FirstPerson/Blueprints/BP_FirstPersonCharacter.Ammo` 0 _asbp_first_person_character)
          (`GameplayStatics.PlaySoundAtLocation` "/Game/VericalSlice/SoundEffects/SFX_Gunshot.SFX_Gunshot" (0.0 0.0 0.0) (struct) 0.3 0.7 0.0 null null null null)
          (`KismetSystemLibrary.Delay` 0.2)
          (`SkeletalMeshComponent.PlayAnimation` (`/Game/FirstPerson/Blueprints/BP_FirstPersonCharacter.SkeletalMesh_Gun` _asbp_first_person_character) "/Game/VericalSlice/Characters/Player/Animation/Fire/A_Player_Fire_Anim.A_Player_Fire_Anim" false)
          (bind _outhits (`KismetSystemLibrary.LineTraceMulti` :`Start` _location :`End` (+ _location (* _rotation 18000.0)) :`TraceChannel` "TraceTypeQuery1" :`DrawDebugType` "ForDuration" :`TraceColor` (struct :`R` 0.226841 :`G` 1.0 :`A` 1.0) :`TraceHitColor` (struct :`R` 1.0 :`B` 0.079394 :`A` 1.0)))
          (for _array_element _outhits
            (bind (_bblockinghit _binitialoverlap _time _distance _location_2 _impactpoint _normal _impactnormal _physmat _hitactor _hitcomponent) (`GameplayStatics.BreakHitResult` _array_element))
            (`KismetSystemLibrary.PrintString` (`KismetSystemLibrary.GetDisplayName` _hitactor))
            (bind _returnvalue_2 (`AbilitySystemBlueprintLibrary.GetAbilitySystemComponent` _hitactor))
            (`/Engine/EditorBlueprintResources/StandardMacros.IsValid` _returnvalue_2
              (:`Is Valid`
                (if (`ActorComponent.ComponentHasTag` _hitcomponent "Headshot")
                  (bind _asbp_first_person_character_2 (cast `/Game/FirstPerson/Blueprints/BP_FirstPersonCharacter` _returnvalue))
                  (set `/Game/FirstPerson/Blueprints/BP_FirstPersonCharacter.HitEnemy` true _asbp_first_person_character_2)
                  (set `/Game/FirstPerson/Blueprints/BP_FirstPersonCharacter.HeadShot` true _asbp_first_person_character_2)
                  (`GameplayStatics.PlaySoundAtLocation` "/Game/VericalSlice/SoundEffects/bell-122093.bell-122093" (0.0 0.0 0.0) (struct) 0.3 1.0 0.0 null null null null)
                  (else
                    (bind _asbp_first_person_character_3 (cast `/Game/FirstPerson/Blueprints/BP_FirstPersonCharacter` _returnvalue))
                    (set `/Game/FirstPerson/Blueprints/BP_FirstPersonCharacter.HitEnemy` true _asbp_first_person_character_3)))
                (bind _returnvalue_3 (`AbilitySystemBlueprintLibrary.GetAbilitySystemComponent` _asbp_first_person_character_3))
                (`AbilitySystemComponent.BP_ApplyGameplayEffectToTarget` :`self` _returnvalue_3 :`GameplayEffectClass` "/Game/GameplayAbilitySystem/Effects/GE_Damage.GE_Damage_C" :`Target` _returnvalue_2 :`Level` 1.0)
                (`AbilitySystemComponent.BP_ApplyGameplayEffectToTarget` :`self` _returnvalue_3 :`GameplayEffectClass` "/Game/GameplayAbilitySystem/Effects/GE_Damage.GE_Damage_C" :`Target` _returnvalue_3 :`Level` 1.0))))
          (`self.K2_EndAbility`)
          (else
            (goto _label)))))
    (:`CastFailed`
      (`self.K2_EndAbility`))))