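; BP_Laser is a boss laser effect actor that traces forward every frame and damages the player it hits.
; While the trace hits the player, each tick applies GE_LaserDamage to the player's cached Ability System Component and calls PostHitProcess.
; The trace result drives the beam endpoint and impact effect.
; Beam length snaps to blocking hits and otherwise grows over time up to a cap, so it visibly extends.
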(event `self.ReceiveBeginPlay`
  (bind _asbp_player_character (cast `/Game/Production/Player/Character/BP_PlayerCharacter` (`GameplayStatics.GetPlayerCharacter` 0)))
  (bind _output_get (set `self.PlayerRef` _asbp_player_character))
  (set `self.GameplayAbilitySystem` (`AbilitySystemBlueprintLibrary.GetAbilitySystemComponent` _output_get)))

(event `self.ReceiveTick`
  (params (DeltaSeconds :type "Float (single-precision)"))
  (bind _returnvalue (`self.K2_GetActorLocation`))
  (bind _returnvalue_2 (+ _returnvalue (* (`self.GetActorForwardVector`) (`self.Distance`))))
  (`|ExecutionSequence`
    (:`then_0`
      (set `self.TraceEnd` _returnvalue_2)
      (bind _outhit (`KismetSystemLibrary.LineTraceSingle` :`Start` _returnvalue :`End` _returnvalue_2 :`TraceChannel` "TraceTypeQuery2" :`DrawDebugType` "ForOneFrame"))
      (cast `/Game/Production/Player/Character/BP_PlayerCharacter` (`.HitActor` (`GameplayStatics.BreakHitResult` _outhit))
        (:`then`
          (if (`KismetSystemLibrary.IsValid` (`self.GameplayAbilitySystem`))
            (`AbilitySystemComponent.BP_ApplyGameplayEffectToSelf` :`self` (`self.GameplayAbilitySystem`) :`GameplayEffectClass` "/Game/Production/GameplayAbilitySystem/Effeects/GE_LaserDamage.GE_LaserDamage_C" :`Level` 1.0)
            (`PlayerCharacter.PostHitProcess` (`self.PlayerRef`))
            (set `self.Bhit` (`GameplayStatics.BreakHitResult` _outhit) :!label _label)
            (set `self.Hit Location` (`.Location` (`GameplayStatics.BreakHitResult` _outhit)))
            (`FXSystemComponent.SetVectorParameter` (`self.Laser`) "LaserEnd" (select `bool` (`self.Bhit`) :`false` (`self.TraceEnd`) :`true` (`self.Hit Location`)))
            (`SceneComponent.SetVisibility` (`self.LaserImpact`) (`self.Bhit`) false)
            (`SceneComponent.K2_SetWorldLocation` (`self.LaserImpact`) (`self.Hit Location`) false false)
            (if (`self.Bhit`)
              (set `self.Distance` (`KismetMathLibrary.VSize` (- (`self.Hit Location`) (`self.K2_GetActorLocation`)))))))
        (:`CastFailed`
          (goto _label))))
    (:`then_1`
      (if (< (`self.Distance`) 5000.0)
        (set `self.Distance` (+ (`self.Distance`) (* DeltaSeconds 9000.0)))))))

(fn `UserConstructionScript`)