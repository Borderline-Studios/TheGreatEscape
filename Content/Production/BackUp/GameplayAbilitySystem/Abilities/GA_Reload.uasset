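; Gameplay ability that reloads the first-person player's gun, ending immediately if the character is meleeing or shooting.
; It finds the character through player pawn 0, flags it as reloading, swaps the gun mesh for a reload mesh, and plays the animation and sound.
; After a fixed delay, not an animation callback, it refills ammo, restores the gun mesh, ends the ability and clears the flag.
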(event `self.K2_ActivateAbility`
  (bind _asbp_first_person_character (cast `/Game/Production/BackUp/BP_FirstPersonCharacter` (`GameplayStatics.GetPlayerPawn` 0))
    (:`then`
      (if (or (`/Game/Production/BackUp/BP_FirstPersonCharacter.IsMelee` _asbp_first_person_character) (`/Game/Production/BackUp/BP_FirstPersonCharacter.IsShooting` _asbp_first_person_character))
        (`self.K2_EndAbility`)
        (else
          (set `/Game/Production/BackUp/BP_FirstPersonCharacter.IsReloading` true _asbp_first_person_character)
          (bind _skeletalmesh_gun (`/Game/Production/BackUp/BP_FirstPersonCharacter.SkeletalMesh_Gun` _asbp_first_person_character))
          (`SceneComponent.SetVisibility` _skeletalmesh_gun false false)
          (bind _skeletalmesh_reload (`/Game/Production/BackUp/BP_FirstPersonCharacter.SkeletalMesh_Reload` _asbp_first_person_character))
          (`SceneComponent.SetVisibility` _skeletalmesh_reload true false)
          (`SkeletalMeshComponent.PlayAnimation` _skeletalmesh_reload "/Game/Production/Player/Animation/Reload/A_Player_Reload_Anim.A_Player_Reload_Anim" false)
          (`GameplayStatics.PlaySoundAtLocation` "/Game/Production/SoundEffects/SFX_Reload.SFX_Reload" (`Actor.K2_GetActorLocation` _asbp_first_person_character) (struct) 0.3 1.0 0.0 null null null null)
          (`KismetSystemLibrary.Delay` (`KismetMathLibrary.SafeDivide` 3.1 1.7))
          (set `/Game/Production/BackUp/BP_FirstPersonCharacter.Ammo` 6 _asbp_first_person_character)
          (`SceneComponent.SetVisibility` _skeletalmesh_gun true false)
          (`SceneComponent.SetVisibility` _skeletalmesh_reload false false)
          (`self.K2_EndAbility` :!label _label)
          (set `/Game/Production/BackUp/BP_FirstPersonCharacter.IsReloading` false _asbp_first_person_character))))
    (:`CastFailed`
      (goto _label))))