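; BP_GameCompleteTrigger is an overlap actor that ends the game with a victory screen when the player reaches it.
; On BeginPlay it caches the first actor of the game mode's default pawn class as the player reference.
; When that actor overlaps it, it disables the BP_PlayerCharacter's collision and movement, zeroes its velocity, and adds WBP_VictoryScreen to the viewport.
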(event `self.ReceiveBeginPlay`
  (bind _returnvalue (`GameplayStatics.GetActorOfClass` (`GameModeBase.DefaultPawnClass` (`GameplayStatics.GetGameMode`))))
  (set `self.PlayerRef` _returnvalue))

(event `self.ReceiveActorBeginOverlap`
  (params (OtherActor :type "Actor Object Reference"))
  (if (== OtherActor (`self.PlayerRef`))
    (bind _asbp_player_character (cast `/Game/Production/Player/Character/BP_PlayerCharacter` (`self.PlayerRef`)))
    (`self.SetActorEnableCollision` _asbp_player_character false)
    (bind _charactermovement (`Character.CharacterMovement` _asbp_player_character))
    (`CharacterMovementComponent.DisableMovement` _charactermovement)
    (set `MovementComponent.Velocity` (0.0 0.0 0.0) _charactermovement)
    (bind _returnvalue (`|CreateWidget` "/Game/Production/UI/VictoryScreen/WBP_VictoryScreen.WBP_VictoryScreen_C"))
    (`UserWidget.AddToViewport` _returnvalue 0)))

(fn `UserConstructionScript`)