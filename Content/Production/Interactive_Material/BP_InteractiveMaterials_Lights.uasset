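; Interactive-material lights Blueprint that keeps the colour of its lights matched to a GlowColour vector parameter.
; UpdateLightsColour reads the parameter and applies it as an sRGB light colour to a point light and two other light components.
; The update runs in the construction script and again every Tick, so the lights follow changes to the parameter.
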(event `self.ReceiveTick`
  (params (DeltaSeconds :type "Float (single-precision)"))
  (`self.UpdateLightsColour`))

(fn `UpdateLightsColour`
  (for _array_element (`|MakeArray` (`self.PointLightComponent`) (`self.LightComponent1`) (`self.LightComponent2`))
    (bind _returnvalue (`KismetMaterialLibrary.GetVectorParameterValue` null "GlowColour"))
    (`LightComponent.SetLightColor` _array_element _returnvalue true)))

(fn `UserConstructionScript`
  (`self.UpdateLightsColour`))