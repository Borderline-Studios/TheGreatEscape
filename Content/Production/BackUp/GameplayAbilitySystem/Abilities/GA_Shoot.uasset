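; GA_Shoot is the first-person player's gameplay ability for firing the gun, blocked while reloading, shooting or in melee.
; With ammo, it plays fire feedback, spends a round and line-traces from the camera view.
; Targets with an ability system receive GE_Damage and award score, with headshot-tagged components adding points and a sound but identical damage.
; After a short delay, it auto-reloads an empty gun, clears the shooting state and ends.
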(event `self.K2_ActivateAbility`
  (bind _returnvalue (`GameplayStatics.GetPlayerPawn` 0))
  (bind (_location _rotation) (`Controller.GetPlayerViewPoint` (`GameplayStatics.GetPlayerController` 0)))
  (bind _asbp_first_person_character (cast `/Game/Production/BackUp/BP_FirstPersonCharacter` (`GameplayStatics.GetPlayerPawn` 0))
    (:`then`
      (if (or (`/Game/Production/BackUp/BP_FirstPersonCharacter.IsReloading` _asbp_first_person_character) (`/Game/Production/BackUp/BP_FirstPersonCharacter.IsShooting` _asbp_first_person_character) (`/Game/Production/BackUp/BP_FirstPersonCharacter.IsMelee` _asbp_first_person_character))
        (`self.K2_EndAbility`)
        (else
          (set `/Game/Production/BackUp/BP_FirstPersonCharacter.IsShooting` true _asbp_first_person_character)
          (bind _ammo (`/Game/Production/BackUp/BP_FirstPersonCharacter.Ammo` _asbp_first_person_character))
          (if (> _ammo 0)
            (`GameplayStatics.PlaySoundAtLocation` "/Game/Production/SoundEffects/SFX_Gunshot.SFX_Gunshot" (`Actor.K2_GetActorLocation` _asbp_first_person_character) (struct) 0.1 (* 1.0 (`GameplayStatics.GetGlobalTimeDilation`)) 0.0 null null null null)
            (`SkeletalMeshComponent.PlayAnimation` (`/Game/Production/BackUp/BP_FirstPersonCharacter.SkeletalMesh_Gun` _asbp_first_person_character) "/Game/Production/Player/Animation/Fire/A_Player_Fire_Anim.A_Player_Fire_Anim" false)
            (`/Engine/EditorBlueprintResources/StandardMacros.DecrementInt` _ammo
              (:`  `
                (bind _outhit (`KismetSystemLibrary.LineTraceSingle` :`Start` _location :`End` (+ _location (* _rotation 18000.0)) :`TraceChannel` "TraceTypeQuery2" :`bTraceComplex` true :`DrawTime` 1.0))
                (bind (_bblockinghit _binitialoverlap _time _distance _location_2 _impactpoint _normal _impactnormal _physmat _hitactor _hitcomponent) (`GameplayStatics.BreakHitResult` _outhit))
                (bind _returnvalue_2 (`AbilitySystemBlueprintLibrary.GetAbilitySystemComponent` _hitactor))
                (`/Engine/EditorBlueprintResources/StandardMacros.IsValid` _returnvalue_2
                  (:`Is Valid`
                    (if (`ActorComponent.ComponentHasTag` _hitcomponent "Headshot")
                      (bind _asbp_first_person_character_2 (cast `/Game/Production/BackUp/BP_FirstPersonCharacter` _returnvalue))
                      (set `/Game/Production/BackUp/BP_FirstPersonCharacter.HitEnemy` true _asbp_first_person_character_2)
                      (set `/Game/Production/BackUp/BP_FirstPersonCharacter.HeadShot` true _asbp_first_person_character_2)
                      (set `/Game/Production/BackUp/BP_FirstPersonCharacter.Score` (+ (`/Game/Production/BackUp/BP_FirstPersonCharacter.Score` _asbp_first_person_character_2) 20) _asbp_first_person_character_2)
                      (`GameplayStatics.PlaySoundAtLocation` "/Game/Production/SoundEffects/SFX_Hit_01_Cue.SFX_Hit_01_Cue" _location_2 (struct) 0.2 2.5 0.0 null null null null)
                      (else
                        (bind _asbp_first_person_character_3 (cast `/Game/Production/BackUp/BP_FirstPersonCharacter` _returnvalue))
                        (set `/Game/Production/BackUp/BP_FirstPersonCharacter.HitEnemy` true _asbp_first_person_character_3)
                        (set `/Game/Production/BackUp/BP_FirstPersonCharacter.Score` (+ (`/Game/Production/BackUp/BP_FirstPersonCharacter.Score` _asbp_first_person_character_3) 10) _asbp_first_person_character_3)))
                    (`AbilitySystemComponent.BP_ApplyGameplayEffectToSelf` :`self` _returnvalue_2 :`GameplayEffectClass` "/Game/Production/BackUp/GameplayAbilitySystem/Effects/GE_Damage.GE_Damage_C" :`Level` 1.0)
                    (`GameplayStatics.PlaySoundAtLocation` "/Game/Production/SoundEffects/SFX_Hit_01.SFX_Hit_01" _location_2 (struct) 1.0 1.0 0.0 null null null null))
                  (:`Is Not Valid`
                    _)))))
          (`KismetSystemLibrary.Delay` 0.3 :!label _label)
          (if (<= (`/Game/Production/BackUp/BP_FirstPersonCharacter.Ammo` _asbp_first_person_character) 0)
            (`/Game/Production/BackUp/BP_FirstPersonCharacter.AutoReload` _asbp_first_person_character))
          (set `/Game/Production/BackUp/BP_FirstPersonCharacter.IsShooting` false _asbp_first_person_character)
          (`self.K2_EndAbility`))))
    (:`CastFailed`
      (goto _label))))