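; Turret drone enemy that charges up and fires a hitscan shot at the player, with a continuously spinning rotor.
; Detection sphere overlaps set InRange and start the charge timer or stop tracking, through functions defined outside this graph.
; Charge cues play Niagara effects and sounds that rise in pitch with each call.
; The shot resets pitch, line-traces to the player camera and, on a hit, draws a tracer and applies GAS damage.
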(event `self.CheckLineToPlayer`
  (bind _returnvalue (`SceneComponent.K2_GetComponentLocation` (`self.TraceSphere`)))
  (bind _asbp_player_character (cast `/Game/Production/Player/Character/BP_PlayerCharacter` (`GameplayStatics.GetPlayerPawn` 0)))
  (set `self.PitchMod` 0.0)
  (bind _outhit (`KismetSystemLibrary.LineTraceSingle` (`SceneComponent.K2_GetComponentLocation` (`self.TraceSphere`)) (`SceneComponent.K2_GetComponentLocation` (`PlayerCharacter.FirstPersonCameraComponent` _asbp_player_character)) "TraceTypeQuery2" true))
  (if (== (`.HitActor` (`GameplayStatics.BreakHitResult` _outhit)) _asbp_player_character)
    (`GameplayStatics.PlaySoundAtLocation` "/Game/Production/SoundEffects/Drone/SFX_Drone_Shoot_02.SFX_Drone_Shoot_02" _returnvalue (struct) 0.3 1.0 0.0 null null null null)
    (bind _returnvalue_2 (`NiagaraFunctionLibrary.SpawnSystemAtLocation` "/Game/Production/Effects/Enemies/Drone/BulletTracer/N_Tracer_System.N_Tracer_System" _returnvalue))
    (`FXSystemComponent.SetVectorParameter` _returnvalue_2 "BeamEnd" (`SceneComponent.K2_GetComponentLocation` (`/Game/Production/Player/Character/BP_PlayerCharacter.LockOnPoint` _asbp_player_character)))
    (bind _returnvalue_3 (`AbilitySystemBlueprintLibrary.GetAbilitySystemComponent` _asbp_player_character))
    (`AbilitySystemComponent.BP_ApplyGameplayEffectToTarget` :`self` _returnvalue_3 :`GameplayEffectClass` "/Game/Production/BackUp/GameplayAbilitySystem/Effects/GE_DroneDamage.GE_DroneDamage_C" :`Target` _returnvalue_3)
    (`PlayerCharacter.PostHitProcess` _asbp_player_character)))

(event `self.LazerTracePlayer`
  (bind _pitchmod (`self.PitchMod`))
  (bind _tracesphere (`self.TraceSphere`))
  (`NiagaraFunctionLibrary.SpawnSystemAttached` "/Game/Production/Effects/Enemies/Drone/ChargeUp/NS_ChargeUp.NS_ChargeUp" _tracesphere "None" (0.0 0.0 0.0) (struct) "SnapToTarget" true)
  (`GameplayStatics.PlaySoundAtLocation` "/Game/Production/Enemies/Blueprints/BomberDrone/SFX/DroneChargeUpSFX.DroneChargeUpSFX" (`SceneComponent.K2_GetComponentLocation` _tracesphere) (struct) 0.3 _pitchmod 0.0 null null null null)
  (set `self.PitchMod` (+ _pitchmod 0.3)))

(event `self.ReceiveTick`
  (params (DeltaSeconds :type "Float (single-precision)"))
  (bind _rotormesh (`self.RotorMesh`))
  (bind (_returnvalue_roll _returnvalue_pitch _returnvalue_yaw) (`KismetMathLibrary.BreakRotator` (`SceneComponent.K2_GetComponentRotation` _rotormesh)))
  (`SceneComponent.K2_SetWorldRotation` _rotormesh (`KismetMathLibrary.MakeRotator` 0.0 0.0 (+ _returnvalue_yaw 5.0)) false false))

(event `self.DetectionSphere.OnComponentBeginOverlap`
  (params (OverlappedComponent :type "PrimitiveComponent Object Reference") (OtherActor :type "Actor Object Reference") (OtherComp :type "PrimitiveComponent Object Reference") (OtherBodyIndex :type Integer) (bFromSweep :type Boolean) (SweepResult :type "HitResult Structure (by ref)"))
  (bind _returnvalue (`self.GetPlayerReference`))
  (if (== _returnvalue OtherActor)
    (set `self.bInRange` true)
    (`self.ChargeSystemTimer`)))

(event `self.DetectionSphere.OnComponentEndOverlap`
  (params (OverlappedComponent :type "PrimitiveComponent Object Reference") (OtherActor :type "Actor Object Reference") (OtherComp :type "PrimitiveComponent Object Reference") (OtherBodyIndex :type Integer))
  (bind _returnvalue (`self.GetPlayerReference`))
  (if (== _returnvalue OtherActor)
    (set `self.bInRange` false)
    (`self.StopTrackPlayer`)))

(fn `UserConstructionScript`)