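; BP_EnemySpawnerRanged is a spawner that creates waves of enemies, ranged by its name, at its own location.
; On BeginPlay it binds SpawnEnemy to the respawn event of BP_TheGreatEscapeGameMode.
; Each call spawns the current count of actors, then raises the increment and adds it to the count, so waves grow at an accelerating rate.
; The NewRound parameter is unused.
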(event `self.ReceiveBeginPlay`
  (bind _asbp_the_great_escape_game_mode (cast `/Game/VericalSlice/Core/GameModes/BP_TheGreatEscapeGameMode` (`GameplayStatics.GetGameMode`)))
  (add `/Game/VericalSlice/Core/GameModes/BP_TheGreatEscapeGameMode.RespawnEnemy` _asbp_the_great_escape_game_mode (delegate `SpawnEnemy`)))

(event `SpawnEnemy`
  (params (NewRound :type Boolean))
  (for _ (range (`self.EnemySpawned`))
    (`|SpawnActorFromClass` "/Game/Enemies/BP_EnemyRanged.BP_EnemyRanged_C" (`self.GetTransform`) "Undefined" "OverrideRootScale" null null))
  (`/Engine/EditorBlueprintResources/StandardMacros.IncrementInt` (`self.EnemyIncrement`)
    (:`  `
      (set `self.EnemySpawned` (+ (`self.EnemySpawned`) (`self.EnemyIncrement`))))))

(fn `UserConstructionScript`)