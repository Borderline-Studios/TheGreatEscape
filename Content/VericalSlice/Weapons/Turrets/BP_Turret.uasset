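; Auto-targeting turret that shoots projectiles at nearby pawns, ignoring the player.
; Each tick it picks the closest pawn in sensing range with line of sight and turns toward it at constant speed with clamped pitch.
; Once off cooldown and nearly facing the target, a DoN loop fires a three-volley burst, staggering left and right guns, cycling muzzle sockets and starting curve-driven recoil timelines.
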(event `self.ReceiveBeginPlay`
  (bind _asbp_first_person_character (cast `/Game/FirstPerson/Blueprints/BP_FirstPersonCharacter` (`GameplayStatics.GetPlayerCharacter` 0)))
  (set `self.Player` _asbp_first_person_character)
  (`TimelineComponent.SetFloatCurve` (`self.RecoilTimelineL`) "/Game/VericalSlice/Weapons/Turrets/RecoilCurve.RecoilCurve" "Recoil")
  (`TimelineComponent.SetFloatCurve` (`self.RecoilTimelineR`) "/Game/VericalSlice/Weapons/Turrets/RecoilCurve.RecoilCurve" "Recoil"))

(event `self.ReceiveTick`
  (params (DeltaSeconds :type "Float (single-precision)"))
  (`self.FindBestTarget`)
  (`self.Target`
    (:`then`
      (`self.UpdateRotation` DeltaSeconds)
      (`self.UpdateFire`))
    (:`else`)))

(event `Fire`
  (set `self.TimeOfLastFire` (`KismetSystemLibrary.GetGameTimeInSeconds`))
  (`|ExecutionSequence`
    (:`then_0`
      (goto _label :!via `Reset`))
    (:`then_1`
      (`/Engine/EditorBlueprintResources/StandardMacros.Do N` 3 :!label _label
        (:`Exit`
          (`|SpawnActorFromClass` "/Game/VericalSlice/Weapons/Turrets/BP_TurretProjectile.BP_TurretProjectile_C" (`SceneComponent.GetSocketTransform` (`self.Turret_RotatingPiece_L`) (`KismetStringLibrary.Conv_StringToName` (`KismetStringLibrary.Concat_StrStr` "FireSocket" (`KismetStringLibrary.Conv_IntToString` (`self.SocketNum`)))) "RTS_World") "Undefined" "OverrideRootScale" null null)
          (`TimelineComponent.PlayFromStart` (`self.RecoilTimelineL`))
          (`KismetSystemLibrary.Delay` 0.2)
          (`|SpawnActorFromClass` "/Game/VericalSlice/Weapons/Turrets/BP_TurretProjectile.BP_TurretProjectile_C" (`SceneComponent.GetSocketTransform` (`self.Turret_RotatingPiece_R`) (`KismetStringLibrary.Conv_StringToName` (`KismetStringLibrary.Concat_StrStr` "FireSocket" (`KismetStringLibrary.Conv_IntToString` (`self.SocketNum`)))) "RTS_World") "Undefined" "OverrideRootScale" null null)
          (`TimelineComponent.PlayFromStart` (`self.RecoilTimelineR`))
          (`/Engine/EditorBlueprintResources/StandardMacros.IncrementInt` (`self.SocketNum`)
            (:`  `
              (if (> (`self.SocketNum`) 3)
                (set `self.SocketNum` 1))
              (`KismetSystemLibrary.Delay` 0.2)
              (goto _label))))))))

(fn `FindBestTarget`
  (locals (BestDistanceLocal :type "Float (double-precision)") (CurrentDistanceLocal :type "Float (double-precision)") (BestTargetLocal :type "Actor Object Reference") (CurrentTargetLocal :type "Actor Object Reference"))
  (set `local.BestDistanceLocal` (+ (`self.SensingRange`) 1.0))
  (bind _outactors (`KismetSystemLibrary.SphereOverlapActors` (`self.K2_GetActorLocation`) (`self.SensingRange`) (`|MakeArray` "ObjectTypeQuery3" :!type "EObjectTypeQuery Enum") null (`|MakeArray` (`self.Player`) :!type "Actor Object Reference")))
  (for _array_element _outactors
    (bind _output_get (set `local.CurrentTargetLocal` _array_element))
    (bind _output_get_2 (set `local.CurrentDistanceLocal` (`self.GetDistanceTo` _output_get self)))
    (if (or (< _output_get_2 (`local.BestDistanceLocal`)) (not (`KismetSystemLibrary.IsValid` (`local.BestTargetLocal`))))
      (bind _result (`self.HasLineOfSight` (`SceneComponent.K2_GetComponentLocation` (`self.Turret_Bottom`)) (`self.K2_GetActorLocation` (`local.CurrentTargetLocal`)) (`|MakeArray` self (`local.CurrentTargetLocal`) :!type "Actor Object Reference")))
      (if _result
        (set `local.BestTargetLocal` (`local.CurrentTargetLocal`))
        (set `local.BestDistanceLocal` (`local.CurrentDistanceLocal`)))))
  (set `self.Target` (`local.BestTargetLocal`)))

(fn `HasLineOfSight`
  (params (From :type "Vector Structure") (To :type "Vector Structure") (ActorsToIgnore :type "Array of Actor Object Reference (by ref)"))
  (returns (Result :type Boolean))
  (bind (_outhit _returnvalue) (`KismetSystemLibrary.LineTraceSingle` From To "TraceTypeQuery1" false ActorsToIgnore "None" false))
  (return (not _returnvalue)))

(fn `UpdateFire`
  (if (> (- (`KismetSystemLibrary.GetGameTimeInSeconds`) (`self.TimeOfLastFire`)) (`self.RateOfFire`))
    (if (> (`KismetMathLibrary.Dot_VectorVector` (`KismetMathLibrary.GetDirectionUnitVector` (`SceneComponent.K2_GetComponentLocation` (`self.Turret_Top`)) (`self.K2_GetActorLocation` (`self.Target`))) (`SceneComponent.GetForwardVector` (`self.Turret_Top`))) 0.99)
      (`self.Fire`))))

(fn `UpdateRotation`
  (params (DeltaSeconds :type "Float (double-precision)"))
  (locals (NewRotation :type "Rotator Structure" :default (struct)))
  ;[1 1 1] Clamp pitch and set world rotation of the turret
  (bind _output_get (set `local.NewRotation` (`KismetMathLibrary.RInterpTo_Constant` (`SceneComponent.K2_GetComponentRotation` (`self.Turret_Top`)) (`KismetMathLibrary.FindLookAtRotation` (`SceneComponent.K2_GetComponentLocation` (`self.Turret_Top`)) (`self.K2_GetActorLocation` (`self.Target`))) (`local.DeltaSeconds`) (`self.RotationSpeed`))))
  (`SceneComponent.K2_SetWorldRotation` (`self.Turret_Top`) (`KismetMathLibrary.MakeRotator` (.roll _output_get) (`KismetMathLibrary.ClampAngle` (.pitch _output_get) -45.0 75.0) (.yaw _output_get)) false false))

(fn `UserConstructionScript`)