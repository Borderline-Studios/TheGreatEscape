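; BP_FloorBlade is a saw hazard that shuttles along a spline and damages the player on contact.
; A timeline moves it along its BP_FloorBladePath, defaulting to one found in the level, and reverses at each end while flipping the mesh's spin.
; Box overlap applies the GE_BladeDamage gameplay effect through the player's ability system and triggers their hit post-process.
; An attached looping-style active sound starts at BeginPlay.
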(event `self.ReceiveBeginPlay`
  ;[1 1 1] If a path was not set default to one
  (`MovementComponent.SetUpdatedComponent` (`self.RotatingMovement`) (`self.Mesh`))
  (if (not (`KismetSystemLibrary.IsValid` (`self.FloorBladePath`)))
    (bind _returnvalue (`GameplayStatics.GetActorOfClass` "/Game/Production/Enemies/FloorBlade/BP_FloorBladePath.BP_FloorBladePath_C"))
    (set `self.FloorBladePath` _returnvalue))
  (`self.MoveBlade`)
  (bind _asbp_player_character (cast `/Game/Production/Player/Character/BP_PlayerCharacter` (`GameplayStatics.GetPlayerCharacter` 0)))
  (bind _output_get (set `self.PlayerRef` _asbp_player_character))
  (set `self.GameplayAbilityComp` (`AbilitySystemBlueprintLibrary.GetAbilitySystemComponent` _output_get))
  (`GameplayStatics.SpawnSoundAttached` "/Game/Production/SoundEffects/FloorBlade/SFX_FloorBlade_Active_01.SFX_FloorBlade_Active_01" null "None" (0.0 0.0 0.0) (struct) "KeepRelativeOffset" true 0.5 1.0 0.0 "/Game/Production/Enemies/Audio/BP_ThrusterAttenuation.BP_ThrusterAttenuation" null))

(event `MoveBlade`
  (bind _spline (`/Game/Production/Enemies/FloorBlade/BP_FloorBladePath.Spline` (`self.FloorBladePath`)))
  (`TimelineComponent.SetPlayRate` (`self.MoveBladeT`) (/ 1.0 (`self.TimeToComplete`)))
  (bind (_direction _movetrack) (`Timeline|MoveBladeT` :!label _label)
    (:`Update`
      (bind _returnvalue (`KismetMathLibrary.Lerp` (`self.LerpStart`) (`SplineComponent.GetSplineLength` _spline) _movetrack))
      (`self.K2_SetActorTransform` (`KismetMathLibrary.MakeTransform` (`SplineComponent.GetLocationAtDistanceAlongSpline` _spline _returnvalue "World") (`SplineComponent.GetRotationAtDistanceAlongSpline` _spline _returnvalue "Local"))))
    (:`Finished`
      (if (`self.TimelineFactor`)
        (`self.SwapDirection` true)
        (goto _label :!via `ReverseFromEnd`)
        (else
          (`self.SwapDirection` false)
          (goto _label :!via `PlayFromStart`))))))

(event `SwapDirection`
  (params (TLFactor :type Boolean))
  (bind _rotatingmovement (`self.RotatingMovement`))
  (if TLFactor
    (set `self.TimelineFactor` false)
    (set `self.LerpStart` 1.0)
    (set `RotatingMovementComponent.RotationRate` (`KismetMathLibrary.MakeRotator` 0.0 (`self.RotationRateY`)) _rotatingmovement)
    (else
      (set `self.TimelineFactor` true)
      (set `self.LerpStart` 0.0)
      (set `RotatingMovementComponent.RotationRate` (`KismetMathLibrary.MakeRotator` 0.0 (* (`self.RotationRateY`) -1.0)) _rotatingmovement))))

(event `self.Box.OnComponentBeginOverlap`
  (params (OverlappedComponent :type "PrimitiveComponent Object Reference") (OtherActor :type "Actor Object Reference") (OtherComp :type "PrimitiveComponent Object Reference") (OtherBodyIndex :type Integer) (bFromSweep :type Boolean) (SweepResult :type "HitResult Structure (by ref)"))
  ;[1 1 1] Damage player if they touch the saw
  (cast `/Game/Production/Player/Character/BP_PlayerCharacter` OtherActor)
  (if (`KismetSystemLibrary.IsValid` (`self.GameplayAbilityComp`))
    (`AbilitySystemComponent.BP_ApplyGameplayEffectToSelf` :`self` (`self.GameplayAbilityComp`) :`GameplayEffectClass` "/Game/Production/GameplayAbilitySystem/Effeects/GE_BladeDamage.GE_BladeDamage_C" :`Level` 1.0)
    (`PlayerCharacter.PostHitProcess` (`self.PlayerRef`))))

(fn `UserConstructionScript`)