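; BP_BossDeath is a boss death effect actor that scatters the boss's body and base parts, then removes itself.
; The construction script gathers the parts into BossParts; BeginPlay gives them one shared dynamic fading material and random impulses.
; After a delay, the BodyFlicker timeline sets that material's Opacity to a constant zero on each update, then destroys the actor on finish.
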(event `self.ReceiveBeginPlay`
  (bind _returnvalue (`KismetMathLibrary.RandomFloatInRange` (`self.MinImpulseVal`) (`self.MaxImpulseVal`)))
  (bind _returnvalue_2 (`KismetMaterialLibrary.CreateDynamicMaterialInstance` "/Game/Production/Enemies/Materials/M_FadingMatBoss.M_FadingMatBoss"))
  (bind _output_get (set `self.FadingMat` _returnvalue_2))
  (for _array_element (`self.BossParts`)
    (`PrimitiveComponent.SetMaterial` _array_element 0 _output_get)
    (`PrimitiveComponent.AddImpulse` _array_element (`KismetMathLibrary.MakeVector` _returnvalue _returnvalue _returnvalue) "None" false))
  (`KismetSystemLibrary.Delay` 4.0)
  (`Timeline|BodyFlicker`
    (:`Update`
      (`MaterialInstanceDynamic.SetScalarParameterValue` (`self.FadingMat`) "Opacity" 0.0))
    (:`Finished`
      (`self.K2_DestroyActor`))))

(fn `UserConstructionScript`
  (set `self.BossParts` (`|MakeArray` (`self.HandR`) (`self.ForeArmR`) (`self.Neck`) (`self.Body`) (`self.ArmR`) (`self.HandL`) (`self.ForeArmL`) (`self.ArmL`) (`self.BasePole`) (`self.BaseConsole`) (`self.BaseBox`) (`self.BasePart`) (`self.Base`) (`self.Head`))))