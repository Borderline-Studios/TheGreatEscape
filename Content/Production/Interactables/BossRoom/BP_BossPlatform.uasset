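; BP_BossPlatform is a boss room platform actor that moves between an activated and a deactivated position.
; On BeginPlay it snaps to the deactivated position.
; ActivatePlatform and DeactivatePlatform events each play a timeline that lerps the actor's location between the two positions without sweeping.
; When the deactivate timeline finishes, the platform destroys itself, so deactivation is final.
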(event `DeactivatePlatform`
  (bind (_direction _newtrack_0) (`Timeline|Deactivate`)
    (:`Update`
      (`self.K2_SetActorLocation` (`KismetMathLibrary.VLerp` (`self.ActivatedPosition`) (`self.DeactiavtedPosition`) _newtrack_0)))
    (:`Finished`
      (`self.K2_DestroyActor`))))

(event `ActivatePlatform`
  (bind (_direction _newtrack_0) (`Timeline|Activate`)
    (:`Update`
      (`self.K2_SetActorLocation` (`KismetMathLibrary.VLerp` (`self.DeactiavtedPosition`) (`self.ActivatedPosition`) _newtrack_0)))))

(event `self.ReceiveBeginPlay`
  (`self.K2_SetActorLocation` (`self.DeactiavtedPosition`)))

(fn `UserConstructionScript`)