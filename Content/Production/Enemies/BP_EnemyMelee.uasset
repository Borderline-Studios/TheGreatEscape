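; Melee robot enemy that turns to face the player and attacks when the player enters its detection sphere.
; Uses GAS for default attributes and damage, with Tick driving a delayed attack and cooldown loop that halts then restores walk speed.
; When its checked attribute hits zero, it ragdolls, credits a kill and updates the GameMode's alive-enemy count, which it incremented on spawn.
; A headshot sphere is attached to the head socket.
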(event `self.ReceiveBeginPlay`
  (`SceneComponent.K2_AttachToComponent` (`self.HeadShotSphere`) (`self.Mesh`) "Base-HumanHead" "SnapToTarget" "SnapToTarget" "SnapToTarget" true)
  ;[1 1 1] When spawned in, increase amount of enemies alive
  (`AbilitySystemComponent.BP_ApplyGameplayEffectToSelf` :`self` (`self.AbilitySystemComponent`) :`GameplayEffectClass` "/Game/GameplayAbilitySystem/Effects/GE_EnemyDefaults.GE_EnemyDefaults_C")
  (bind _asbp_the_great_escape_game_mode (cast `/Game/VericalSlice/Core/GameModes/BP_TheGreatEscapeGameMode` (`GameplayStatics.GetGameMode`)))
  (`/Engine/EditorBlueprintResources/StandardMacros.IncrementInt` (`/Game/VericalSlice/Core/GameModes/BP_TheGreatEscapeGameMode.NumOfEnemiesAlive` _asbp_the_great_escape_game_mode)
    (:`  `
      (bind _asbp_first_person_character (cast `/Game/Production/BackUp/BP_FirstPersonCharacter` (`GameplayStatics.GetPlayerCharacter` 0)))
      (set `self.PlayerRef` _asbp_first_person_character)
      (set `self.StoppingDistance` 75.0)
      (`KismetSystemLibrary.Delay` (`KismetMathLibrary.RandomFloatInRange` 0.0 0.4))
      (`GameplayStatics.PlaySoundAtLocation` "/Game/VericalSlice/SoundEffects/SFX_Robot_Noise.SFX_Robot_Noise" (`self.K2_GetActorLocation` (`self.PlayerRef`)) (struct) 0.3 1.0 0.0 null null null null))))

(event `self.ReceiveTick`
  (params (DeltaSeconds :type "Float (single-precision)"))
  ;[1 1 1] Check if enemy is dead, if so kill it
  (`self.Look at Player` DeltaSeconds)
  (if (<= (`.ReturnValue` (`AbilitySystemComponent.GetGameplayAttributeValue` (`self.AbilitySystemComponent`) (struct :`AttributeName` "Health" :`Attribute` "/Script/TheGreatEscape.GASAttributeSet:Health" :`AttributeOwner` "Class'\"/Script/TheGreatEscape.GASAttributeSet\"'"))) 0.0)
    (if (not (`self.bDying`))
      (set `self.bDying` true)
      (`self.Ragdoll`))
    (else
      ;[1 1 1] Melee Attack functionality
      (if (`self.bIsCoolingDown`)
        (set `self.bIsCoolingDown` false)
        (`KismetSystemLibrary.Delay` (`self.coolDownAmount`))
        (set `CharacterMovementComponent.MaxWalkSpeed` 600.0 (`self.CharacterMovement`))
        (if (`self.bInAttackRange`)
          (set `self.bCanAttack` true))
        (elif (`self.bCanAttack`)
          (set `self.bIsAttacking` true)
          (`self.Attacking`)
          (`KismetSystemLibrary.PrintString` "attacking")
          (else
            (set `self.bCanAttack` false)))))))

(event `Ragdoll`
  ;[1 1 1] Ragdoll - do physics object stuff on character
  (`PrimitiveComponent.SetSimulatePhysics` (`self.Mesh`) true)
  (`CharacterMovementComponent.DisableMovement` (`self.CharacterMovement`))
  (`self.SetLifeSpan` self 3.0)
  (`/Engine/EditorBlueprintResources/StandardMacros.IncrementInt` (`/Game/Production/BackUp/BP_FirstPersonCharacter.Kills` (`self.PlayerRef`))
    (:`  `
      (`KismetSystemLibrary.Delay` 2.5)
      (bind _asbp_the_great_escape_game_mode (cast `/Game/VericalSlice/Core/GameModes/BP_TheGreatEscapeGameMode` (`GameplayStatics.GetGameMode`)))
      (`/Engine/EditorBlueprintResources/StandardMacros.DecrementInt` (`/Game/VericalSlice/Core/GameModes/BP_TheGreatEscapeGameMode.NumOfEnemiesAlive` _asbp_the_great_escape_game_mode)
        (:`  `
          (`/Game/VericalSlice/Core/GameModes/BP_TheGreatEscapeGameMode.CheckNumOfEnemyLeft` _asbp_the_great_escape_game_mode))))))

(event `self.PlayerAttackDetection.OnComponentBeginOverlap`
  (params (OverlappedComponent :type "PrimitiveComponent Object Reference") (OtherActor :type "Actor Object Reference") (OtherComp :type "PrimitiveComponent Object Reference") (OtherBodyIndex :type Integer) (bFromSweep :type Boolean) (SweepResult :type "HitResult Structure (by ref)"))
  ;[1 1 1] On overlap of attack sphere - can attack
  (cast `/Game/Production/BackUp/BP_FirstPersonCharacter` OtherActor)
  (set `self.bCanAttack` true)
  (set `self.bInAttackRange` true))

(event `self.PlayerAttackDetection.OnComponentEndOverlap`
  (params (OverlappedComponent :type "PrimitiveComponent Object Reference") (OtherActor :type "Actor Object Reference") (OtherComp :type "PrimitiveComponent Object Reference") (OtherBodyIndex :type Integer))
  ;[1 1 1] On overlap end of attack sphere - can no longer attack
  (cast `/Game/Production/BackUp/BP_FirstPersonCharacter` OtherActor)
  (set `self.bCanAttack` false)
  (set `self.bInAttackRange` false))

(event `Attacking`
  ;[1 1 1] Attack function
  (`KismetSystemLibrary.Delay` 0.5)
  (`AbilitySystemComponent.BP_ApplyGameplayEffectToTarget` :`self` (`self.AbilitySystemComponent`) :`GameplayEffectClass` "/Game/GameplayAbilitySystem/Effects/GE_EnemyDamage.GE_EnemyDamage_C" :`Target` (`AbilitySystemBlueprintLibrary.GetAbilitySystemComponent` (`self.PlayerRef`)))
  (set `CharacterMovementComponent.MaxWalkSpeed` 0.0 (`self.CharacterMovement`))
  (`KismetSystemLibrary.PrintString` "attacking player")
  (set `self.bIsCoolingDown` true)
  (set `self.bCanAttack` false)
  (`KismetSystemLibrary.Delay` 1.0)
  (set `self.bIsAttacking` false))

(fn `Look at Player`
  (params (DeltaSeconds :type "Float (double-precision)"))
  (bind (_returnvalue_roll _returnvalue_pitch _returnvalue_yaw) (`KismetMathLibrary.BreakRotator` (`KismetMathLibrary.RInterpTo_Constant` (`self.K2_GetActorRotation`) (`KismetMathLibrary.FindLookAtRotation` (`self.K2_GetActorLocation`) (`self.K2_GetActorLocation` (`self.PlayerRef`))) (`self.Delta Seconds`) (`self.RotationSpeed`))))
  (set `self.Delta Seconds` DeltaSeconds)
  (`self.K2_SetActorRotation` (`KismetMathLibrary.MakeRotator` 0.0 0.0 _returnvalue_yaw)))

(fn `UserConstructionScript`)