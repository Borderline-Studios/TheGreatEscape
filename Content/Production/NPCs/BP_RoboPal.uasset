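; BP_RoboPal is a robot NPC that wakes when the player enters its WakeRange and goes back to sleep when the player leaves.
; Waking plays a timeline that lifts it from its start position with a 360-degree yaw offset, then a second timeline bobs it up and down by alternating play and reverse.
; Leaving clears IsAwake to suspend the bob and plays a sleep timeline back to the initial location and rotation.
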(event `self.ReceiveBeginPlay`
  (bind _output_get (set `self.InitLocation` (`self.K2_GetActorLocation`)))
  (set `self.LocAfterWake` (+ _output_get (0.0 0.0 50.0)))
  (bind _output_get_2 (set `self.InitRot` (`self.K2_GetActorRotation`)))
  (set `self.newRot` (`KismetMathLibrary.MakeRotator` (.roll _output_get_2) (.pitch _output_get_2) (+ (.yaw _output_get_2) 360.0))))

(event `self.WakeRange.OnComponentBeginOverlap`
  (params (OverlappedComponent :type "PrimitiveComponent Object Reference") (OtherActor :type "Actor Object Reference") (OtherComp :type "PrimitiveComponent Object Reference") (OtherBodyIndex :type Integer) (bFromSweep :type Boolean) (SweepResult :type "HitResult Structure (by ref)"))
  (cast `/Game/Production/Player/Character/BP_PlayerCharacter` OtherActor)
  (bind (_direction _newtrack_0) (`Timeline|TL_Wake`)
    (:`Update`
      (`self.K2_SetActorLocationAndRotation` (`KismetMathLibrary.VLerp` (`self.InitLocation`) (`self.LocAfterWake`) _newtrack_0) (`KismetMathLibrary.RLerp` (`self.InitRot`) (`self.newRot`) _newtrack_0)))
    (:`Finished`
      ;[1 1 1] Repeat lerping up & down
      (set `self.IsAwake` true)
      (set `self.TimelineFactor` true)
      (set `self.LerpLoc` (+ (`self.LocAfterWake`) (0.0 0.0 70.0)))
      (bind (_direction_2 _newpos) (`Timeline|TL_RoboFriend` :!via `PlayFromStart` :!label _label)
        (:`Update`
          (if (`self.IsAwake`)
            (`self.K2_SetActorLocation` (`KismetMathLibrary.VLerp` (`self.LocAfterWake`) (`self.LerpLoc`) _newpos))))
        (:`Finished`
          (if (`self.TimelineFactor`)
            (set `self.TimelineFactor` false)
            (goto _label :!via `ReverseFromEnd`)
            (else
              (set `self.TimelineFactor` true)
              (goto _label :!via `PlayFromStart`))))))))

(event `self.WakeRange.OnComponentEndOverlap`
  (params (OverlappedComponent :type "PrimitiveComponent Object Reference") (OtherActor :type "Actor Object Reference") (OtherComp :type "PrimitiveComponent Object Reference") (OtherBodyIndex :type Integer))
  (cast `/Game/Production/Player/Character/BP_PlayerCharacter` OtherActor)
  (set `self.IsAwake` false)
  (bind (_direction _newtrack_0) (`Timeline|TlSleep` :!via `PlayFromStart`)
    (:`Update`
      (`self.K2_SetActorLocationAndRotation` (`KismetMathLibrary.VLerp` (`self.K2_GetActorLocation`) (`self.InitLocation`) _newtrack_0) (`KismetMathLibrary.RLerp` (`self.newRot`) (`self.InitRot`) _newtrack_0)))))

(fn `UserConstructionScript`)