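; Pushable radio-style button actor that blends the global GlowColour in MPC_InteractiveMaterials toward its own GoalColour.
; Hover highlights via custom primitive data; its test line-traces the mesh from screen centre, but returns false as written.
; Left-mouse release while hovered pushes it and releases every other button of its class.
; Tick interpolates AnimProgress, sliding the mesh between two locations and driving the colour blend for the current button.
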(event `self.ReceiveBeginPlay`
  (`self.SetCurrentLocation` (`self.AnimProgress`)))

(event `self.ReceiveTick`
  (params (DeltaSeconds :type "Float (single-precision)"))
  (bind _animprogress (`self.AnimProgress`))
  (`|ExecutionSequence`
    (:`then_0`
      (bind _ishovered (`self.IsHoveredByCursor`))
      ;[1 1 1] Highlight material when hovered by cursor
      (`PrimitiveComponent.SetCustomPrimitiveDataFloat` (`self.StaticMeshComponent`) 0 (`KismetMathLibrary.SelectFloat` 1.0 0.0 _ishovered))
      (if _ishovered
        ;[1 1 1] Was mouse just pressed?
        (if (`PlayerController.WasInputKeyJustReleased` (`GameplayStatics.GetPlayerController` 0) "LeftMouseButton")
          (`|ExecutionSequence`
            (:`then_0`
              ;[1 1 1] Start animating towards a pushed state
              (set `self.IsAnimating` true)
              (set `self.IsGoalDirectionDown` true)
              (set `self.IsCurrentButton` true))
            (:`then_1`
              ;[1 1 1] Un-push all other buttons
              (bind _outactors (`GameplayStatics.GetAllActorsOfClass` (`GameplayStatics.GetObjectClass` self)))
              (for _array_element _outactors
                (if (!= _array_element self)
                  (set `/Game/Essentials/Blueprints/BP_GameplayMaterials_Button.IsAnimating` true _array_element)
                  (set `/Game/Essentials/Blueprints/BP_GameplayMaterials_Button.IsGoalDirectionDown` false _array_element)
                  (set `/Game/Essentials/Blueprints/BP_GameplayMaterials_Button.IsCurrentButton` false _array_element))))))))
    (:`then_1`
      (if (`self.IsAnimating`)
        ;[1 1 1] Update animation
        (`|ExecutionSequence`
          (:`then_0`
            (set `self.AnimProgress` (`KismetMathLibrary.FInterpTo_Constant` (`self.AnimProgress`) (`KismetMathLibrary.SelectFloat` 1.0 0.0 (`self.IsGoalDirectionDown`)) DeltaSeconds (`self.AnimSpeed`))))
          (:`then_1`
            (`self.SetCurrentLocation` (`self.AnimProgress`)))
          (:`then_2`
            (if (`self.IsCurrentButton`)
              ;;[1 1 1] Control global color
              (bind _returnvalue (`KismetMaterialLibrary.GetVectorParameterValue` "/Game/Interactive_Material/MaterialFunctions/MPC_InteractiveMaterials.MPC_InteractiveMaterials" "GlowColour"))
              (`KismetMaterialLibrary.SetVectorParameterValue` "/Game/Interactive_Material/MaterialFunctions/MPC_InteractiveMaterials.MPC_InteractiveMaterials" "GlowColour" (`KismetMathLibrary.LinearColorLerp` _returnvalue (`self.GoalColour`) (`self.AnimProgress`))))))))
    (:`then_2`
      ;[1 1 1] Stop animation
      (if (or (and (== (`self.IsGoalDirectionDown`) false) (`KismetMathLibrary.NearlyEqual_FloatFloat` _animprogress)) (and (== (`self.IsGoalDirectionDown`) true) (`KismetMathLibrary.NearlyEqual_FloatFloat` _animprogress 1.0)))
        (set `self.IsAnimating` false)))))

(fn `InitializeVariables`)

(fn `IsHoveredByCursor`
  (returns (IsHovered :type Boolean))
  (bind _returnvalue (`WidgetLayoutLibrary.GetPlayerScreenWidgetGeometry` (`GameplayStatics.GetPlayerController` 0)))
  (bind (_returnvalue_x _returnvalue_y) (`KismetMathLibrary.BreakVector2D` (`SlateBlueprintLibrary.GetAbsoluteSize` _returnvalue)))
  (bind (_worldlocation _worlddirection) (`PlayerController.DeprojectScreenPositionToWorld` (`GameplayStatics.GetPlayerController` 0) (/ _returnvalue_x 2.0) (/ _returnvalue_y 2.0)))
  (`PrimitiveComponent.K2_LineTraceComponent` (`self.StaticMeshComponent`) _worldlocation (+ _worldlocation (* _worlddirection (`self.HoverDistanceFromPlayerMax`))) false false false)
  (return false))

(fn `SetCurrentLocation`
  (params (Progress :type "Float (double-precision)"))
  (`SceneComponent.K2_SetRelativeLocation` (`self.StaticMeshComponent`) (`KismetMathLibrary.VLerp` (`self.LocationMin`) (`self.LocationMax`) Progress) false true))

(fn `StartAnimation`
  (set `self.IsAnimating` true)
  (set `self.IsGoalDirectionDown` (not (`self.IsGoalDirectionDown`))))

(fn `UserConstructionScript`
  (`self.SetCurrentLocation` (`self.AnimProgress`)))