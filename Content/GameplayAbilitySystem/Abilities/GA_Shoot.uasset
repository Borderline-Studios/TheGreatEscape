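; Gameplay ability that fires the first-person player's pistol as a hitscan shot, blocked while reloading.
; With ammo left, it spends a round, plays fire animation and time-dilation-pitched sound, then line-traces from the camera view.
; Targets with an ability system flag a hit on the character: "Headshot"-tagged components set HeadShot and ring a bell, others receive GE_Damage.
; A short delay then ends the ability and restores the idle animation.
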(event `self.K2_ActivateAbility`
  (bind _returnvalue (`GameplayStatics.GetPlayerPawn` 0))
  (bind (_location _rotation) (`Controller.GetPlayerViewPoint` (`GameplayStatics.GetPlayerController` 0)))
  (bind _asbp_first_person_character (cast `/Game/FirstPerson/Blueprints/BP_FirstPersonCharacter` (`GameplayStatics.GetPlayerPawn` 0))
    (:`then`
      (if (`/Game/FirstPerson/Blueprints/BP_FirstPersonCharacter.IsReloading` _asbp_first_person_character)
        (`self.K2_EndAbility`)
        (else
          (bind _ammo (`/Game/FirstPerson/Blueprints/BP_FirstPersonCharacter.Ammo` _asbp_first_person_character))
          (if (> _ammo 0)
            (`SkeletalMeshComponent.PlayAnimation` (`/Game/FirstPerson/Blueprints/BP_FirstPersonCharacter.Gun` _asbp_first_person_character) "/Game/VericalSlice/Characters/Player/Animation/Fire/A_Player_Fire_Anim.A_Player_Fire_Anim" false)
            (`/Engine/EditorBlueprintResources/StandardMacros.DecrementInt` _ammo
              (:`  `
                (`GameplayStatics.PlaySoundAtLocation` "/Game/VericalSlice/SoundEffects/9mm-pistol-shoot-short-reverb-7152.9mm-pistol-shoot-short-reverb-7152" (`Actor.K2_GetActorLocation` _asbp_first_person_character) (struct) 0.3 (`GameplayStatics.GetGlobalTimeDilation`) 0.0 null null null null)
                (bind _outhit (`KismetSystemLibrary.LineTraceSingle` :`Start` _location :`End` (+ _location (* _rotation 18000.0)) :`TraceChannel` "TraceTypeQuery2" :`bTraceComplex` true :`DrawTime` 1.0))
                (bind (_bblockinghit _binitialoverlap _time _distance _location_2 _impactpoint _normal _impactnormal _physmat _hitactor _hitcomponent) (`GameplayStatics.BreakHitResult` _outhit))
                (bind _returnvalue_2 (`AbilitySystemBlueprintLibrary.GetAbilitySystemComponent` _hitactor))
                (`/Engine/EditorBlueprintResources/StandardMacros.IsValid` _returnvalue_2
                  (:`Is Valid`
                    (if (`ActorComponent.ComponentHasTag` _hitcomponent "Headshot")
                      (bind _asbp_first_person_character_2 (cast `/Game/FirstPerson/Blueprints/BP_FirstPersonCharacter` _returnvalue))
                      (set `/Game/FirstPerson/Blueprints/BP_FirstPersonCharacter.HitEnemy` true _asbp_first_person_character_2)
                      (set `/Game/FirstPerson/Blueprints/BP_FirstPersonCharacter.HeadShot` true _asbp_first_person_character_2)
                      (`GameplayStatics.PlaySoundAtLocation` "/Game/VericalSlice/SoundEffects/bell-122093.bell-122093" _location_2 (struct) 0.3 1.0 0.0 null null null null)
                      (else
                        (bind _asbp_first_person_character_3 (cast `/Game/FirstPerson/Blueprints/BP_FirstPersonCharacter` _returnvalue))
                        (set `/Game/FirstPerson/Blueprints/BP_FirstPersonCharacter.HitEnemy` true _asbp_first_person_character_3)
                        (`AbilitySystemComponent.BP_ApplyGameplayEffectToTarget` :`self` (`AbilitySystemBlueprintLibrary.GetAbilitySystemComponent` _asbp_first_person_character_3) :`GameplayEffectClass` "/Game/GameplayAbilitySystem/Effects/GE_Damage.GE_Damage_C" :`Target` _returnvalue_2))))
                  (:`Is Not Valid`
                    _)))))
          (`KismetSystemLibrary.Delay` 0.3 :!label _label)
          (`self.K2_EndAbility`)
          (`SkeletalMeshComponent.PlayAnimation` (`/Game/FirstPerson/Blueprints/BP_FirstPersonCharacter.Gun` _asbp_first_person_character) "/Game/VericalSlice/Characters/Player/Animation/Idle/A_Player_Idle_Anim.A_Player_Idle_Anim" false))))
    (:`CastFailed`
      (goto _label))))