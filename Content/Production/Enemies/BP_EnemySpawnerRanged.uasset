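; BP_EnemySpawnerRanged is a placeable spawner that creates BP_EnemyRanged enemies at its own transform when the game mode signals an enemy respawn.
; On BeginPlay it binds SpawnEnemy to the respawn event of BP_TheGreatEscapeGameMode.
; Each call spawns EnemySpawned enemies, then raises that count by EnemyIncrement, so waves grow linearly until a new-round flag resets both values.
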(event `self.ReceiveBeginPlay`
  (bind _asbp_the_great_escape_game_mode (cast `/Game/Production/GameMode/BP_TheGreatEscapeGameMode` (`GameplayStatics.GetGameMode`)))
  (add `/Game/Production/GameMode/BP_TheGreatEscapeGameMode.RespawnEnemy` _asbp_the_great_escape_game_mode (delegate `SpawnEnemy`)))

(event `SpawnEnemy`
  (params (NewRound :type Boolean))
  (if NewRound
    (set `self.EnemySpawned` 1)
    (set `self.EnemyIncrement` 1))
  (for _ (range (`self.EnemySpawned`))
    (`|SpawnActorFromClass` "/Game/Production/Enemies/BP_EnemyRanged.BP_EnemyRanged_C" (`self.GetTransform`) "Undefined" "OverrideRootScale" null null))
  (set `self.EnemySpawned` (+ (`self.EnemySpawned`) (`self.EnemyIncrement`))))

(fn `UserConstructionScript`)