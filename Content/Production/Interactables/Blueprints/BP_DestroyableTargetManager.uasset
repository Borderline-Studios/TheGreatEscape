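; Destroyable target Blueprint that counts hits and moves linked actors once the required total is reached.
; Each destroy event spawns sparks, turns the target mesh material red, increments the hit count and checks it.
; A timeline lerps one actor, optionally a second, from its current location each update toward finish locations.
; When it finishes, a class check gates enabling collision on a moved ladder.
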(event `CheckTargetsHit`
  (bind _actortotrigger (`self.ActorToTrigger`))
  (bind _secondactortotrigger (`self.SecondActorToTrigger`))
  (if (>= (`self.CurrentHits`) (`self.TotalHits`))
    (bind (_direction _alpha) (`Timeline|Timeline_0`)
      (:`Update`
        (`self.K2_SetActorLocation` _actortotrigger (`KismetMathLibrary.VLerp` (`self.K2_GetActorLocation` _actortotrigger) (`self.FinishLocation`) _alpha) false false)
        (if (`self.SecondActor`)
          (`self.K2_SetActorLocation` _secondactortotrigger (`KismetMathLibrary.VLerp` (`self.K2_GetActorLocation` _secondactortotrigger) (`self.Actor2FinishLocation`) _alpha) false false)))
      (:`Finished`
        (if (`self.CheckIfMovingLadder`)
          (bind _asbp_ladder (cast `/Game/Production/Interactables/LevelTraversal/BP_Ladder` (`self.ActorToTrigger`)))
          (`/Game/Production/Interactables/LevelTraversal/BP_Ladder.EnableCollision` _asbp_ladder))))))

(event `self.DestoryTarget`
  (`NiagaraFunctionLibrary.SpawnSystemAtLocation` "/Game/Production/Effects/Enemies/Hit_Kill/NS_SheildSparks.NS_SheildSparks" (`SceneComponent.K2_GetComponentLocation` (`self.TargetMesh`)) (struct) (0.5 0.5 0.5))
  (`PrimitiveComponent.SetMaterial` (`self.TargetMesh`) 1 "/Game/Production/Enviroment/Interactables/Target/MI_TargetRed.MI_TargetRed")
  (set `self.CurrentHits` (+ (`self.CurrentHits`) 1.0))
  (`self.CheckTargetsHit`))

(fn `CheckIfMovingLadder`
  (returns (IsLadder :type Boolean))
  (bind _actortotrigger (`self.ActorToTrigger`))
  (return (and (`KismetSystemLibrary.IsValid` _actortotrigger) (== (`GameplayStatics.GetObjectClass` _actortotrigger) null))))

(fn `UserConstructionScript`)