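; First-person player character Blueprint that handles the presentation side of the revolver and rifle shooter.
; Events spawn HUD, checkpoint, damage-number and rocket-target UI, toggle the hit vignette, lerp FOV, reapply GAS default effects and reload the level.
; BeginPlay attaches muzzle spheres to the weapons, and Tick shows sight VFX while aiming.
; Escape pauses through zero time dilation, while hardcoded Z/X/C and K/L keys jump levels and toggle boss platforms.
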(event `self.HitVignette`
  (bind _postprocess (`self.PostProcess`))
  (`SceneComponent.SetVisibility` _postprocess true false)
  (`ActorComponent.Activate` _postprocess true))

(event `ActivateCheckPointUI`
  (`/Game/Production/UI/WidgetBlueprints/WBP_PlayerUI.PlayCheckpointAnim` (`self.UIRef`)))

(event `self.ApplyUI`
  (bind _returnvalue (`|CreateWidget` "/Game/Production/UI/WidgetBlueprints/WBP_PlayerUI.WBP_PlayerUI_C" (`GameplayStatics.GetPlayerController` 0)))
  (`UserWidget.AddToViewport` _returnvalue 0))

(event `self.ReApplyPassives`
  (`AbilitySystemComponent.BP_ApplyGameplayEffectToSelf` :`self` (`self.AbilitySystemComponent`) :`GameplayEffectClass` "/Game/Production/BackUp/GameplayAbilitySystem/Effects/GE_PlayerDefaults.GE_PlayerDefaults_C")
  (`self.PostHitProcess`))

(event `self.RocketTargetWidget`
  (params (InActor :type "Actor Object Reference"))
  (bind _returnvalue (`|CreateWidget` "/Game/Production/UI/WidgetBlueprints/WBP_RocketTarget.WBP_RocketTarget_C" null InActor))
  (bind _output_get (set `self.RocketTargetUI` _returnvalue))
  (`UserWidget.AddToViewport` _output_get 0))

(event `self.RemoveRocketTargetWidget`
  (`Widget.RemoveFromParent` (`self.RocketTargetUI`)))

(event `Key|Escape` :consume false
  (params (Key :type "Key Structure"))
  (bind _returnvalue (`GameplayStatics.GetPlayerController` 0))
  (:`Pressed`
    (if (not (`self.bGamePaused`))
      (`GameplayStatics.SetGlobalTimeDilation` 0.0)
      (set `self.bGamePaused` true)
      (bind _returnvalue_2 (`|CreateWidget` "/Game/Production/UI/WidgetBlueprints/WBP_PauseMenu.WBP_PauseMenu_C"))
      (bind _output_get (set `self.PauseUI` _returnvalue_2))
      (`UserWidget.AddToViewport` _output_get 0)
      (`WidgetBlueprintLibrary.SetInputMode_UIOnlyEx` _returnvalue (`self.PauseUI`))
      (set `PlayerController.bShowMouseCursor` true _returnvalue))))

(event `self.CreateDamageWidget`
  (params (HitResult :type "HitResult Structure") (Damage :type "Float (single-precision)") (ShieldDamage :type Boolean))
  (bind _returnvalue (`|CreateWidget` "/Game/Production/UI/WidgetBlueprints/WBP_DamageNumbers.WBP_DamageNumbers_C" null Damage (`.HitActor` (`GameplayStatics.BreakHitResult` HitResult)) ShieldDamage))
  (`UserWidget.AddToViewport` _returnvalue 0))

(event `self.LerpFOV`
  (params (From :type "Float (single-precision)") (To :type "Float (single-precision)") (Reverse :type Boolean))
  (if Reverse
    (bind (_direction _alpha) (`Timeline|Timeline_0` :!via `ReverseFromEnd` :!label _label)
      (:`Update`
        (`CameraComponent.SetFieldOfView` (`self.FirstPersonCameraComponent`) (`KismetMathLibrary.Lerp` From To _alpha))))
    (else
      (goto _label :!via `PlayFromStart`))))

(event `self.CallVignette`
  (bind _postprocess (`self.PostProcess`))
  (`SceneComponent.SetVisibility` _postprocess true false)
  (`ActorComponent.Activate` _postprocess true))

(event `self.ResetLevel`
  (bind _returnvalue (`GameplayStatics.GetCurrentLevelName` true))
  (`GameplayStatics.OpenLevel` (`KismetStringLibrary.Conv_StringToName` _returnvalue)))

(event `self.DisableVignette`
  (bind _postprocess (`self.PostProcess`))
  (`SceneComponent.SetVisibility` _postprocess false false)
  (`ActorComponent.Deactivate` _postprocess))

(event `self.ReceiveBeginPlay`
  (`SceneComponent.SetVisibility` (`self.PostProcess`) false false)
  (`SceneComponent.K2_AttachToComponent` (`self.MuzzleSphere`) (`self.RevolverMesh1P`) "Bone_Chamber" "KeepWorld" "SnapToTarget" "KeepWorld" true)
  (`SceneComponent.K2_AttachToComponent` (`self.RifleMuzzleSphere`) (`self.RifleMesh1P`) "Trigger" "KeepWorld" "SnapToTarget" "KeepWorld" true)
  (if (`self.AutoApplyUI`)
    (bind _returnvalue (`|CreateWidget` "/Game/Production/UI/WidgetBlueprints/WBP_PlayerUI.WBP_PlayerUI_C" (`GameplayStatics.GetPlayerController` 0)))
    (bind _output_get (set `self.UIRef` _returnvalue))
    (`UserWidget.AddToViewport` _output_get 0)
    (`SceneComponent.SetVisibility` (`self.RevolverMesh1P`) true false)))

(event `self.ReceiveTick`
  (params (DeltaSeconds :type "Float (single-precision)"))
  (bind _sightvfx (`self.SightVFX`))
  (if (`self.bADS`)
    (`SceneComponent.SetVisibility` _sightvfx true false)
    (else
      (`SceneComponent.SetVisibility` _sightvfx false false))))

(event `Key|Z`
  (params (Key :type "Key Structure"))
  (:`Pressed`
    (`GameplayStatics.OpenLevel` "Level_Travel_01")))

(event `Key|X`
  (params (Key :type "Key Structure"))
  (:`Pressed`
    (`GameplayStatics.OpenLevel` "Level_Travel_03")))

(event `Key|C`
  (params (Key :type "Key Structure"))
  (:`Pressed`
    (`GameplayStatics.OpenLevel` "Level_Boss_Arena_01")))

(event `Key|K`
  (params (Key :type "Key Structure"))
  (:`Pressed`
    (bind _outactors (`GameplayStatics.GetAllActorsOfClass` "/Game/Production/Interactables/BossRoom/BP_BossPlatform.BP_BossPlatform_C"))
    (for _array_element _outactors
      (`/Game/Production/Interactables/BossRoom/BP_BossPlatform.ActivatePlatform` _array_element))))

(event `Key|L`
  (params (Key :type "Key Structure"))
  (:`Pressed`
    (bind _outactors (`GameplayStatics.GetAllActorsOfClass` "/Game/Production/Interactables/BossRoom/BP_BossPlatform.BP_BossPlatform_C"))
    (for _array_element _outactors
      (`/Game/Production/Interactables/BossRoom/BP_BossPlatform.DeactivatePlatform` _array_element))))

(fn `UserConstructionScript`)