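; BP_SoundQueTrigger is a trigger volume that plays a sound cue once when the player character enters its box.
; On overlap it stops the player's current AudioComp, spawns SoundToPlay at the player pawn's location and stores the new component on the player, so trigger sounds replace rather than overlap each other.
; The CanPlay flag is cleared on first use, so this Blueprint never fires again by itself.
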(event `self.ReceiveBeginPlay`)

(event `self.Box.OnComponentBeginOverlap`
  (params (OverlappedComponent :type "PrimitiveComponent Object Reference") (OtherActor :type "Actor Object Reference") (OtherComp :type "PrimitiveComponent Object Reference") (OtherBodyIndex :type Integer) (bFromSweep :type Boolean) (SweepResult :type "HitResult Structure (by ref)"))
  (bind _asbp_player_character (cast `/Game/Production/Player/Character/BP_PlayerCharacter` OtherActor))
  (if (`self.CanPlay`)
    (set `self.CanPlay` false)
    (bind _audiocomp (`/Game/Production/Player/Character/BP_PlayerCharacter.AudioComp` _asbp_player_character))
    (if (`KismetSystemLibrary.IsValid` _audiocomp)
      (`AudioComponent.Stop` _audiocomp))
    (bind _returnvalue (`GameplayStatics.SpawnSoundAtLocation` (`self.SoundToPlay`) (`self.K2_GetActorLocation` (`GameplayStatics.GetPlayerPawn` 0)) (struct) 1.0 1.0 0.0 null null))
    (bind _output_get (set `/Game/Production/Player/Character/BP_PlayerCharacter.AudioComp` _returnvalue _asbp_player_character))
    (`AudioComponent.Play` _output_get 0.0)))

(fn `UserConstructionScript`)