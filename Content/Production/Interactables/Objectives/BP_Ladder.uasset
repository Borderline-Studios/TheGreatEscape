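; BP_Ladder is an interactable ladder that automatically carries the player up a spline when they overlap its box.
; It moves the first spline point to the player's closest spline location, then chains two timelines: one centers the player, the other moves them along the spline.
; On completion it restores the spline start and clears the climbing flag; input disabling is unwired, though EnableInput still runs.
; Two functions toggle the box's collision.
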(event `self.ReceiveBeginPlay`
  (bind _returnvalue (`GameplayStatics.GetActorOfClass` "/Game/Production/Player/Character/BP_PlayerCharacter.BP_PlayerCharacter_C"))
  (set `self.PlayerRef` _returnvalue)
  (set `self.SplineStart` (`SplineComponent.GetLocationAtSplinePoint` (`self.PlayerMoveSpline`) 0 "World"))
  (`TimelineComponent.SetPlayRate` (`self.CenterPlayerOnLadder`) 4.0)
  (`TimelineComponent.SetPlayRate` (`self.PlayerAscendLadder`) 1.5))

(event `self.Box.OnComponentBeginOverlap`
  (params (OverlappedComponent :type "PrimitiveComponent Object Reference") (OtherActor :type "Actor Object Reference") (OtherComp :type "PrimitiveComponent Object Reference") (OtherBodyIndex :type Integer) (bFromSweep :type Boolean) (SweepResult :type "HitResult Structure (by ref)"))
  (bind _playerref (`self.PlayerRef`))
  (bind _playermovespline (`self.PlayerMoveSpline`))
  (bind _returnvalue (`self.K2_GetActorLocation` _playerref))
  (bind _returnvalue_2 (`SplineComponent.FindLocationClosestToWorldLocation` (`self.PlayerMoveSpline`) _returnvalue "World"))
  (if (and (== OtherActor _playerref) (not (`self.bPlayerClimbingLadder`)))
    (set `self.bPlayerClimbingLadder` true)
    (set `self.PlayerLerpStart` _returnvalue)
    (set `self.PlayerLerpEnd` _returnvalue_2)
    (`SplineComponent.SetLocationAtSplinePoint` (`self.PlayerMoveSpline`) 0 _returnvalue_2 "World" true)
    (bind (_direction _playerlerptospline) (`Timeline|CenterPlayerOnLadder` :!via `PlayFromStart`)
      (:`Update`
        (`self.K2_SetActorLocation` (`self.PlayerRef`) (`KismetMathLibrary.VLerp` (`self.PlayerLerpStart`) (`self.PlayerLerpEnd`) _playerlerptospline) false false))
      (:`Finished`
        (bind (_direction_2 _playerascendalpha) (`Timeline|PlayerAscendLadder` :!via `PlayFromStart`)
          (:`Update`
            (`self.K2_SetActorLocation` (`self.PlayerRef`) (`SplineComponent.GetLocationAtDistanceAlongSpline` _playermovespline (`KismetMathLibrary.Lerp` 0.0 (`SplineComponent.GetSplineLength` _playermovespline) _playerascendalpha) "World") false false))
          (:`Finished`
            (`self.EnableInput` (`self.PlayerRef`) null)
            (`SplineComponent.SetLocationAtSplinePoint` (`self.PlayerMoveSpline`) 0 (`self.SplineStart`) "World" true)
            (set `self.bPlayerClimbingLadder` false)))))))

(fn `DisableCollision`
  (`PrimitiveComponent.SetCollisionEnabled` (`self.Box`) "NoCollision"))

(fn `EnableCollision`
  (`PrimitiveComponent.SetCollisionEnabled` (`self.Box`) "QueryOnly"))

(fn `UserConstructionScript`)