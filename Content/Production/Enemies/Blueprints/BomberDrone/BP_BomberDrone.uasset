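; Bomber drone enemy that homes in on the player and explodes, with a constantly spinning mesh.
; Entering DetectionSphere sets the homing target and starts a fixed-interval beep; the distance-based BeepTime is never used.
; ExplodeSphere overlap detonates after a short delay, applying a GAS effect to the player with VFX, sound and camera shake.
; Mesh hits reduce HP until it explodes without applying that effect.
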(event `self.ReceiveBeginPlay`
  (bind _asbp_player_character (cast `/Game/Production/Player/Character/BP_PlayerCharacter` (`GameplayStatics.GetPlayerPawn` 0)))
  (set `self.As BP Player Character` _asbp_player_character))

(event `self.ReceiveTick`
  (params (DeltaSeconds :type "Float (single-precision)"))
  (bind (_returnvalue_roll _returnvalue_pitch _returnvalue_yaw) (`KismetMathLibrary.BreakRotator` (`SceneComponent.K2_GetComponentRotation` (`self.StaticMesh1`))))
  (`SceneComponent.K2_SetWorldRotation` (`self.StaticMesh1`) (`KismetMathLibrary.MakeRotator` 0.0 0.0 (+ _returnvalue_yaw 100.0)) false false)
  (set `self.BeepTime` (`KismetMathLibrary.NormalizeToRange` (`KismetMathLibrary.Vector_Distance` (`self.K2_GetActorLocation` (`self.As BP Player Character`)) (`SceneComponent.K2_GetComponentLocation` (`self.DefaultSceneRoot`))) 0.0 1.0)))

(event `CustomEvent_0`
  (`GameplayStatics.PlaySoundAtLocation` "/Game/Production/Enemies/Blueprints/BomberDrone/SFX/BombDroneBeepSFX.BombDroneBeepSFX" (`SceneComponent.K2_GetComponentLocation` (`self.DefaultSceneRoot`)) (struct) 1.0 1.0 0.0 null null null null))

(event `self.DetectionSphere.OnComponentBeginOverlap`
  (params (OverlappedComponent :type "PrimitiveComponent Object Reference") (OtherActor :type "Actor Object Reference") (OtherComp :type "PrimitiveComponent Object Reference") (OtherBodyIndex :type Integer) (bFromSweep :type Boolean) (SweepResult :type "HitResult Structure (by ref)"))
  (bind _flyingmovement (`self.FlyingMovement`))
  (bind _as_bp_player_character (`self.As BP Player Character`))
  (if (== _as_bp_player_character OtherActor)
    (set `ProjectileMovementComponent.HomingTargetComponent` (`Character.CapsuleComponent` _as_bp_player_character) (`self.FlyingMovement`))
    (set `ProjectileMovementComponent.InitialSpeed` (`MovementComponent.GetMaxSpeed` _flyingmovement) _flyingmovement)
    (bind _returnvalue (`KismetSystemLibrary.K2_SetTimerDelegate` (delegate `CustomEvent_0`) 0.5 true))
    (set `self.BeepTimer` _returnvalue)))

(event `self.ExplodeSphere.OnComponentBeginOverlap`
  (params (OverlappedComponent :type "PrimitiveComponent Object Reference") (OtherActor :type "Actor Object Reference") (OtherComp :type "PrimitiveComponent Object Reference") (OtherBodyIndex :type Integer) (bFromSweep :type Boolean) (SweepResult :type "HitResult Structure (by ref)"))
  (bind _as_bp_player_character (`self.As BP Player Character`))
  (bind _returnvalue (`AbilitySystemBlueprintLibrary.GetAbilitySystemComponent` _as_bp_player_character))
  (bind _returnvalue_2 (`SceneComponent.K2_GetComponentLocation` (`self.DefaultSceneRoot`)))
  (`KismetSystemLibrary.Delay` 0.3)
  (if (== (`self.As BP Player Character`) OtherActor)
    (`NiagaraFunctionLibrary.SpawnSystemAtLocation` "/Game/Production/Effects/Enemies/Hit_Kill/NS_Explosion.NS_Explosion" _returnvalue_2)
    (`GameplayStatics.PlaySoundAtLocation` "/Game/Production/Enemies/Blueprints/BomberDrone/SFX/Bomber_ExplodeSFX.Bomber_ExplodeSFX" _returnvalue_2 (struct) 1.0 1.0 0.0 null null null null)
    (`AbilitySystemComponent.BP_ApplyGameplayEffectToTarget` :`self` _returnvalue :`GameplayEffectClass` "/Game/Production/BackUp/GameplayAbilitySystem/Effects/GE_BomberDroneEffect.GE_BomberDroneEffect_C" :`Target` _returnvalue :`Level` 1.0)
    (`PlayerCharacter.PostHitProcess` _as_bp_player_character)
    (`PlayerCameraManager.StartCameraShake` :`self` (`GameplayStatics.GetPlayerCameraManager` 0) :`ShakeClass` "/Game/Production/Player/Character/CameraEffects/ExplosionCamShake.ExplosionCamShake_C" :`Scale` 4.0)
    (`self.K2_DestroyActor`)))

(event `self.DetectionSphere.OnComponentEndOverlap`
  (params (OverlappedComponent :type "PrimitiveComponent Object Reference") (OtherActor :type "Actor Object Reference") (OtherComp :type "PrimitiveComponent Object Reference") (OtherBodyIndex :type Integer))
  (if (== OtherActor (`self.As BP Player Character`))
    (bind _output_get (set `self.BeepTimer` (struct)))
    (`KismetSystemLibrary.K2_ClearAndInvalidateTimerHandle` _output_get)))

(event `self.StaticMesh.OnComponentHit`
  (params (HitComponent :type "PrimitiveComponent Object Reference") (OtherActor :type "Actor Object Reference") (OtherComp :type "PrimitiveComponent Object Reference") (NormalImpulse :type "Vector Structure") (Hit :type "HitResult Structure (by ref)"))
  (bind _hp (`self.HP`))
  (bind _returnvalue (`SceneComponent.K2_GetComponentLocation` (`self.DefaultSceneRoot`)))
  (set `self.HP` (- _hp 10.0))
  (if (<= _hp 0.0)
    (`NiagaraFunctionLibrary.SpawnSystemAtLocation` "/Game/Production/Effects/Enemies/Hit_Kill/NS_Explosion.NS_Explosion" _returnvalue)
    (`GameplayStatics.PlaySoundAtLocation` "/Game/Production/Enemies/Blueprints/BomberDrone/SFX/Bomber_ExplodeSFX.Bomber_ExplodeSFX" _returnvalue (struct) 1.0 1.0 0.0 null null null null)
    (`PlayerCameraManager.StartCameraShake` :`self` (`GameplayStatics.GetPlayerCameraManager` 0) :`ShakeClass` "/Game/Production/Player/Character/CameraEffects/ExplosionCamShake.ExplosionCamShake_C" :`Scale` 4.0)
    (`self.K2_DestroyActor`)))

(fn `UserConstructionScript`)