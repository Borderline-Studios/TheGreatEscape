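; A trigger volume that updates the objective text on the train engine when the player enters it.
; On BeginPlay it finds and caches the BP_TrainEngine and BP_PlayerCharacter actors, printing a message and destroying itself if no train exists.
; A box overlap by the cached player passes NewText to the train's UpdateObjectiveText, gated by a DoOnce so it fires only once.
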(event `self.ReceiveBeginPlay`
  (bind _returnvalue (`GameplayStatics.GetActorOfClass` "/Game/Production/Train/BP_TrainEngine.BP_TrainEngine_C"))
  (bind _output_get (set `self.TrainRef` _returnvalue))
  (if (`KismetSystemLibrary.IsValid` _output_get)
    (bind _returnvalue_2 (`GameplayStatics.GetActorOfClass` "/Game/Production/Player/Character/BP_PlayerCharacter.BP_PlayerCharacter_C"))
    (set `self.PlayerRef` _returnvalue_2)
    (else
      (`KismetSystemLibrary.PrintString` (`KismetStringLibrary.Concat_StrStr` "Train not found, destroying: " (`KismetSystemLibrary.GetDisplayName` null)))
      (`self.K2_DestroyActor`))))

(event `self.Box.OnComponentBeginOverlap`
  (params (OverlappedComponent :type "PrimitiveComponent Object Reference") (OtherActor :type "Actor Object Reference") (OtherComp :type "PrimitiveComponent Object Reference") (OtherBodyIndex :type Integer) (bFromSweep :type Boolean) (SweepResult :type "HitResult Structure (by ref)"))
  (if (== OtherActor (`self.PlayerRef`))
    (`/Engine/EditorBlueprintResources/StandardMacros.DoOnce` false
      (:`Completed`
        (`TrainEngine.UpdateObjectiveText` (`self.TrainRef`) (`self.NewText`))))))

(fn `UserConstructionScript`)