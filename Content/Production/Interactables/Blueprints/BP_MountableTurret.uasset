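; Mountable turret pawn that the player controller possesses when BP_PlayerCharacter overlaps its box, whose collision then turns off; no dismount logic exists.
; Mouse axes aim it, and holding Shoot runs Fire, which re-arms a timer at FireRate rounds per minute until release.
; Each shot plays a random sound, draws a debug camera line trace and applies a GAS damage effect to BP_EnemyRework hits, using the enemy's own ability system as source.
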(event `Fire`
  (bind _camera (`self.Camera`))
  (bind _returnvalue (`SceneComponent.K2_GetComponentLocation` _camera))
  (bind _returnvalue_2 (`KismetSystemLibrary.K2_SetTimerDelegate` (delegate `Fire`) (/ 60.0 (`self.FireRate`))))
  (set `self.GunTimerRef` _returnvalue_2)
  (`GameplayStatics.PlaySoundAtLocation` (`KismetArrayLibrary.Array_Random` (`self.Sound`)) (`SceneComponent.K2_GetComponentLocation` (`self.StaticMesh`)) (struct) 0.3 (`KismetMathLibrary.RandomFloatInRange` 0.9 1.1) 0.0 null null null null)
  (bind _outhit (`KismetSystemLibrary.LineTraceSingle` :`Start` _returnvalue :`End` (+ _returnvalue (* (`SceneComponent.GetForwardVector` _camera) (`self.Range`))) :`TraceChannel` "TraceTypeQuery1" :`DrawDebugType` "ForDuration" :`DrawTime` 0.11))
  (bind _asbp_enemy_rework (cast `/Game/Production/Enemies/Rework/BP_EnemyRework` (`.HitActor` (`GameplayStatics.BreakHitResult` _outhit))))
  (bind _returnvalue_3 (`AbilitySystemBlueprintLibrary.GetAbilitySystemComponent` _asbp_enemy_rework))
  (if (`KismetSystemLibrary.IsValid` _returnvalue_3)
    (`AbilitySystemComponent.BP_ApplyGameplayEffectToTarget` :`self` _returnvalue_3 :`GameplayEffectClass` "/Game/Production/GameplayAbilitySystem/Effeects/GE_Damage_This.GE_Damage_This_C" :`Target` _returnvalue_3 :`Level` 11.0)))

(event `self.Box.OnComponentBeginOverlap`
  (params (OverlappedComponent :type "PrimitiveComponent Object Reference") (OtherActor :type "Actor Object Reference") (OtherComp :type "PrimitiveComponent Object Reference") (OtherBodyIndex :type Integer) (bFromSweep :type Boolean) (SweepResult :type "HitResult Structure (by ref)"))
  (cast `/Game/Production/Player/Character/BP_PlayerCharacter` OtherActor)
  (`Controller.Possess` (`GameplayStatics.GetPlayerController` 0) self)
  (`PrimitiveComponent.SetCollisionEnabled` (`self.Box`) "NoCollision"))

(event `InputAxis|Turn Right / Left Mouse`
  (params (AxisValue :type "Float (single-precision)"))
  (`self.AddControllerYawInput` AxisValue))

(event `InputAction|Shoot`
  (params (Key :type "Key Structure"))
  (:`Pressed`
    (`self.Fire`))
  (:`Released`
    (`KismetSystemLibrary.K2_ClearAndInvalidateTimerHandle` (`self.GunTimerRef`))))

(event `InputAxis|Look Up / Down Mouse`
  (params (AxisValue :type "Float (single-precision)"))
  (`self.AddControllerPitchInput` AxisValue))

(fn `UserConstructionScript`)