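; BP_EnemyReworkDeath is the death effect actor for the reworked enemy, a set of body parts that fly apart and fade out.
; The construction script gathers the body, thruster, arms and head into an array.
; On BeginPlay each part gets a shared dynamic fading material and a random velocity-change impulse.
; After a short delay a flicker timeline drives the material's opacity, then the actor destroys itself.
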(event `self.ReceiveBeginPlay`
  (bind _returnvalue (`KismetMathLibrary.RandomFloatInRange` (`self.MinImpulseVal`) (`self.MaxImpulseVal`)))
  (bind _returnvalue_2 (`KismetMaterialLibrary.CreateDynamicMaterialInstance` "/Game/Production/Enemies/Materials/M_FadingMat.M_FadingMat"))
  (bind _output_get (set `self.FadingMat` _returnvalue_2))
  (for _array_element (`self.BodyParts`)
    (`PrimitiveComponent.SetMaterial` _array_element 0 _output_get)
    (`PrimitiveComponent.AddImpulse` _array_element (`KismetMathLibrary.MakeVector` _returnvalue _returnvalue _returnvalue) "None" true))
  (`KismetSystemLibrary.Delay` 3.0)
  (bind (_direction _bodyflicker) (`Timeline|BodyFlicker` :!via `PlayFromStart`)
    (:`Update`
      (`MaterialInstanceDynamic.SetScalarParameterValue` (`self.FadingMat`) "Opacity" _bodyflicker))
    (:`Finished`
      (`self.K2_DestroyActor`))))

(fn `UserConstructionScript`
  (set `self.BodyParts` (`|MakeArray` (`self.Body`) (`self.Thruster`) (`self.LArm`) (`self.FallApartHead`) (`self.RArm`))))