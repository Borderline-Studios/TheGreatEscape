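; BP_EnergyRibbon is a train effect actor that drives a Niagara energy ribbon from actor transforms.
; Each Tick it rotates the ribbon's owning actor to look at the Sphere's owning actor.
; That Sphere owner's transform acts as a control, with world X setting Length, X scale setting Width and roll setting TwistSpeed.
; The Blueprint's own world Z sets Curve.
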(event `self.ReceiveTick`
  (params (DeltaSeconds :type "Float (single-precision)"))
  (bind (_returnvalue_x _returnvalue_y _returnvalue_z) (`KismetMathLibrary.BreakVector` (`self.K2_GetActorLocation`)))
  (bind _ns_energyribbon (`self.NS_EnergyRibbon`))
  (bind _returnvalue (`ActorComponent.GetOwner` (`self.Sphere`)))
  (bind _returnvalue_2 (`ActorComponent.GetOwner` _ns_energyribbon))
  (bind _returnvalue_x_2 (`KismetMathLibrary.BreakVector` (`self.K2_GetActorLocation` _returnvalue)))
  (bind _returnvalue_x_3 (`KismetMathLibrary.BreakVector` (`self.GetActorScale3D` _returnvalue)))
  (bind _returnvalue_roll (`KismetMathLibrary.BreakRotator` (`self.K2_GetActorRotation` _returnvalue)))
  (`NiagaraComponent.SetVariableFloat` _ns_energyribbon "Length" _returnvalue_x_2)
  (`self.K2_SetActorRotation` _returnvalue_2 (`KismetMathLibrary.FindLookAtRotation` (`self.K2_GetActorLocation` _returnvalue_2) (`self.K2_GetActorLocation` _returnvalue)) false)
  (`NiagaraComponent.SetVariableFloat` _ns_energyribbon "Width" _returnvalue_x_3)
  (`NiagaraComponent.SetVariableFloat` _ns_energyribbon "TwistSpeed" _returnvalue_roll)
  (`NiagaraComponent.SetVariableFloat` _ns_energyribbon "Curve" _returnvalue_z))

(fn `UserConstructionScript`)