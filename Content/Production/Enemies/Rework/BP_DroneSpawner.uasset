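; BP_DroneSpawner is an enemy spawner that creates a batch of BP_EnemyReworkDrone actors when the player enters its trigger sphere.
; BeginPlay sizes the sphere from SpawnTriggerRadius, and a player overlap spawns NumOfDrones, then blocks respawning until SpawnDelay elapses.
; GetRandLocation supplies each spawn transform, but its random X/Y and elevated Z calculations are left unconnected.
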(event `self.ReceiveBeginPlay`
  (`SphereComponent.SetSphereRadius` (`self.CollisionRadius`) (`self.SpawnTriggerRadius`) true))

(event `self.CollisionRadius.OnComponentBeginOverlap`
  (params (OverlappedComponent :type "PrimitiveComponent Object Reference") (OtherActor :type "Actor Object Reference") (OtherComp :type "PrimitiveComponent Object Reference") (OtherBodyIndex :type Integer) (bFromSweep :type Boolean) (SweepResult :type "HitResult Structure (by ref)"))
  (cast `/Game/Production/Player/Character/BP_PlayerCharacter` OtherActor)
  (`KismetSystemLibrary.PrintString` "spawn drones")
  (if (`self.bCanDroneSpawn`)
    (for _ (range (`self.NumOfDrones`))
      (`|SpawnActorFromClass` "/Game/Production/Enemies/Rework/BP_EnemyReworkDrone.BP_EnemyReworkDrone_C" (`KismetMathLibrary.MakeTransform` (`self.GetRandLocation`)) "AdjustIfPossibleButAlwaysSpawn" "OverrideRootScale" null null))
    (set `self.bCanDroneSpawn` false)
    (`self.CanSpawnAgain`)))

(event `CanSpawnAgain`
  (`KismetSystemLibrary.Delay` (`self.SpawnDelay`))
  (set `self.bCanDroneSpawn` true))

(fn `UserConstructionScript`)