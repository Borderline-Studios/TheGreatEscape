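; BP_InteractableDoor is a door that slides open along the world Y axis when its OpenDoor event is called.
; BeginPlay caches the Door component's world location as the closed position and derives the open position at a fixed offset from it.
; OpenDoor plays the LerpPosition timeline, whose alpha interpolates the door between the two positions without sweeping.
; The file has no closing logic and no trigger of its own.
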(event `self.OpenDoor`
  (bind (_direction _alpha) (`Timeline|LerpPosition`)
    (:`Update`
      (`SceneComponent.K2_SetWorldLocation` (`self.Door`) (`KismetMathLibrary.VLerp` (`self.StartPosition`) (`self.FinishPosition`) _alpha) false false))))

(event `self.ReceiveBeginPlay`
  (bind _returnvalue (`SceneComponent.K2_GetComponentLocation` (`self.Door`)))
  (set `self.StartPosition` _returnvalue)
  (set `self.FinishPosition` (- _returnvalue (0.0 100.0 0.0))))

(fn `UserConstructionScript`)