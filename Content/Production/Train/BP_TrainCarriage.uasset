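; BP_TrainCarriage is a train carriage that shows an energy ribbon effect only on the EMP cart variant.
; On the BPNotifyInitialised event, it compares its mesh to the EMP cart mesh reference.
; On a match, it repositions the BP_EnergyRibbon child actor's sphere, rotates the component and sets the Niagara effect's width.
; Otherwise, or if the cast fails, it destroys the ribbon component.
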(event `self.BPNotify_Initialised`
  (bind _bp_energyribbon (`self.BP_EnergyRibbon`))
  (if (== (`StaticMeshComponent.StaticMesh` (`self.CarMesh`)) (`self.EMPCart_MeshRef`))
    (bind _asbp_energy_ribbon (cast `/Game/Production/Effects/Train/EnergyRibbon/BP_EnergyRibbon` (`ChildActorComponent.ChildActor` _bp_energyribbon))
      (:`then`
        (`SceneComponent.K2_SetRelativeLocation` (`/Game/Production/Effects/Train/EnergyRibbon/BP_EnergyRibbon.Sphere` _asbp_energy_ribbon) (320.0 0.0 0.0) false false)
        (`SceneComponent.K2_SetRelativeRotation` _bp_energyribbon (struct :`Yaw` 90.0) false false)
        (`NiagaraComponent.SetVariableFloat` (`/Game/Production/Effects/Train/EnergyRibbon/BP_EnergyRibbon.NS_EnergyRibbon` _asbp_energy_ribbon) "Width" 5.0))
      (:`CastFailed`
        (`ActorComponent.K2_DestroyComponent` _bp_energyribbon :!label _label)))
    (else
      (goto _label))))

(fn `UserConstructionScript`)