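; BP_Enemy is an enemy character that reports its spawn and death to BP_TheGreatEscapeGameMode.
; BeginPlay increments the game mode's living-enemy count.
; As temporary logic, a hit against the first-person character decrements that count, calls CheckNumOfEnemyLeft and destroys the enemy.
; The Ragdoll event is unfinished: it disables movement but turns mesh physics simulation off, and its only caller, a health check, is never run.
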(event `self.ReceiveBeginPlay`
  ;[1 1 1] When spawned in, increase amount of enemies alive
  (bind _asbp_the_great_escape_game_mode (cast `/Game/VericalSlice/Core/GameModes/BP_TheGreatEscapeGameMode` (`GameplayStatics.GetGameMode`)))
  (`/Engine/EditorBlueprintResources/StandardMacros.IncrementInt` (`/Game/VericalSlice/Core/GameModes/BP_TheGreatEscapeGameMode.NumOfEnemiesAlive` _asbp_the_great_escape_game_mode)))

(event `self.ReceiveTick`
  (params (DeltaSeconds :type "Float (single-precision)")))

(event `self.ReceiveHit`
  (params (MyComp :type "PrimitiveComponent Object Reference") (Other :type "Actor Object Reference") (OtherComp :type "PrimitiveComponent Object Reference") (bSelfMoved :type Boolean) (HitLocation :type "Vector Structure") (HitNormal :type "Vector Structure") (NormalImpulse :type "Vector Structure") (Hit :type "HitResult Structure (by ref)"))
  ;[1 1 1] temp
  (cast `/Game/Production/BackUp/BP_FirstPersonCharacter` Other
    (:`then`
      (bind _asbp_the_great_escape_game_mode (cast `/Game/VericalSlice/Core/GameModes/BP_TheGreatEscapeGameMode` (`GameplayStatics.GetGameMode`))
        (:`then`
          (`/Engine/EditorBlueprintResources/StandardMacros.DecrementInt` (`/Game/VericalSlice/Core/GameModes/BP_TheGreatEscapeGameMode.NumOfEnemiesAlive` _asbp_the_great_escape_game_mode)
            (:`  `
              (`/Game/VericalSlice/Core/GameModes/BP_TheGreatEscapeGameMode.CheckNumOfEnemyLeft` _asbp_the_great_escape_game_mode)
              (`self.K2_DestroyActor`))))
        (:`CastFailed`
          (`KismetSystemLibrary.PrintString` "failed game mode"))))
    (:`CastFailed`
      (`KismetSystemLibrary.PrintString` "failed"))))

(event `Ragdoll`
  ;[1 1 1] Ragdoll - do physics object stuff on character
  (`PrimitiveComponent.SetSimulatePhysics` (`self.Mesh`) false)
  (`CharacterMovementComponent.DisableMovement` (`self.CharacterMovement`)))

(fn `UserConstructionScript`)