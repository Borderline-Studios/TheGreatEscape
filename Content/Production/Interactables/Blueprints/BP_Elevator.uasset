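; BP_Elevator is an interactable lever-operated elevator that moves the whole actor between a deactivated and an activated position, starting at the deactivated one.
; Activate toggles GoingUp and plays or reverses the lever rotation timeline, whose completion drives the movement timeline in the matching direction.
; A box trigger shows a widget and enables custom depth on two meshes while the player overlaps, with initial widget visibility checked on BeginPlay.
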(event `self.Activate`
  (if (`self.GoingUp`)
    (set `self.GoingUp` false)
    (bind (_direction _newtrack_0) (`Timeline|LeverLerp` :!via `PlayFromStart` :!label _label)
      (:`Update`
        (`SceneComponent.K2_SetWorldRotation` (`self.StaticMesh2`) (`KismetMathLibrary.RLerp` (struct) (struct :`Roll` 90.0) _newtrack_0) false false))
      (:`Finished`
        (if (`self.GoingUp`)
          (bind (_direction_2 _newtrack_0_2) (`Timeline|Timeline_0` :!via `ReverseFromEnd` :!label _label_2)
            (:`Update`
              (`self.K2_SetActorLocation` (`KismetMathLibrary.VLerp` (`self.DeactiavtedPosition`) (`self.ActivatedPosition`) _newtrack_0_2))))
          (else
            (goto _label_2 :!via `PlayFromStart`)))))
    (else
      (set `self.GoingUp` true)
      (goto _label :!via `ReverseFromEnd`))))

(event `self.ReceiveBeginPlay`
  (`self.K2_SetActorLocation` (`self.DeactiavtedPosition`))
  (bind _returnvalue (`GameplayStatics.GetActorOfClass` "/Game/Production/Player/Character/BP_PlayerCharacter.BP_PlayerCharacter_C"))
  (`SceneComponent.SetVisibility` (`self.Widget`) (`PrimitiveComponent.IsOverlappingActor` (`self.Box`) _returnvalue) false))

(event `self.Box.OnComponentBeginOverlap`
  (params (OverlappedComponent :type "PrimitiveComponent Object Reference") (OtherActor :type "Actor Object Reference") (OtherComp :type "PrimitiveComponent Object Reference") (OtherBodyIndex :type Integer) (bFromSweep :type Boolean) (SweepResult :type "HitResult Structure (by ref)"))
  (cast `/Game/Production/Player/Character/BP_PlayerCharacter` OtherActor)
  (`PrimitiveComponent.SetRenderCustomDepth` (`self.StaticMesh1`) true)
  (`PrimitiveComponent.SetRenderCustomDepth` (`self.StaticMesh2`) true)
  (`SceneComponent.SetVisibility` (`self.Widget`) true false))

(event `self.Box.OnComponentEndOverlap`
  (params (OverlappedComponent :type "PrimitiveComponent Object Reference") (OtherActor :type "Actor Object Reference") (OtherComp :type "PrimitiveComponent Object Reference") (OtherBodyIndex :type Integer))
  (cast `/Game/Production/Player/Character/BP_PlayerCharacter` OtherActor)
  (`PrimitiveComponent.SetRenderCustomDepth` (`self.StaticMesh1`) false)
  (`PrimitiveComponent.SetRenderCustomDepth` (`self.StaticMesh2`) false)
  (`SceneComponent.SetVisibility` (`self.Widget`) false false))

(fn `UserConstructionScript`)