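; Lightning ball effect actor that throws electric arcs onto surrounding surfaces.
; On Tick, after a cooldown, it line traces in a random direction between a min and max radius and spawns an attached Niagara arc on a hit, passing beam endpoints and normal.
; Optional secondary traces chain from each last hit within a random cone around the original direction, spawning secondary arcs until a miss or count limit.
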(event `self.ReceiveTick`
  (params (DeltaSeconds :type "Float (single-precision)"))
  (`self.UpdateTraces`))

(fn `UpdateTraces`
  (locals (RandomDirection :type "Vector Structure" :default (0.0 0.0 0.0)) (ImpactOffset :type "Float (double-precision)" :default 1.0) (LasthitLocation :type "Vector Structure") (LasthitWithOffset :type "Vector Structure") (LasthitNormal :type "Vector Structure"))
  (bind _returnvalue (`self.K2_GetActorLocation`))
  (bind _returnvalue_2 (* (`local.RandomDirection`) (`self.MinRadius`)))
  (bind _returnvalue_3 (+ (`local.LasthitLocation`) (* (`local.LasthitNormal`) (`self.SecondTraceOffset`))))
  ;[1 1 1] Check Cooldown
  (if (>= (- (`GameplayStatics.GetTimeSeconds`) (`self.LastTrace`)) (`self.TraceCooldown`))
    ;[1 1 1] Trace
    (set `local.RandomDirection` (`KismetMathLibrary.RandomUnitVector`))
    (bind _outhit (`KismetSystemLibrary.LineTraceSingle` :`Start` (+ _returnvalue _returnvalue_2) :`End` (+ _returnvalue (* (`local.RandomDirection`) (`self.MaxRadius`))) :`TraceChannel` "TraceTypeQuery1" :`DrawTime` (`self.TraceCooldown`)))
    ;[1 1 1] Reset Cooldown
    (set `self.LastTrace` (`GameplayStatics.GetTimeSeconds`))
    (bind (_bblockinghit _binitialoverlap _time _distance _location _impactpoint _normal _impactnormal) (`GameplayStatics.BreakHitResult` _outhit))
    ;[1 1 1] Spawn Niagara system and set parameters
    (if _bblockinghit
      (`|ExecutionSequence`
        (:`then_0`
          (bind _returnvalue_4 (`NiagaraFunctionLibrary.SpawnSystemAttached` "/Game/Production/Effects/Environment/LightningExplosion/NS_LightningArcs.NS_LightningArcs" (`self.DefaultSceneRoot`) "None" (0.0 0.0 0.0) (struct) "KeepRelativeOffset" true))
          (`NiagaraComponent.SetVariableVec3` _returnvalue_4 "BeamStartPoint" _returnvalue_2)
          (bind _returnvalue_5 (+ _impactpoint (* _impactnormal (`local.ImpactOffset`))))
          (`NiagaraComponent.SetVariableVec3` _returnvalue_4 "BeamEndPoint" _returnvalue_5)
          (`NiagaraComponent.SetVariableVec3` _returnvalue_4 "ImpactNormal" _impactnormal)
          ;[1 1 1] UpdateLasthitInfo
          (set `local.LasthitLocation` _impactpoint)
          (set `local.LasthitWithOffset` _returnvalue_5)
          (set `local.LasthitNormal` _impactnormal))
        (:`then_1`
          (if (`self.SecondTraces`)
            (for _ (range 1 (+ (`self.MaxSecondaryTraces`) 1))
              ;[1 1 1] Secondary Trace
              (bind _outhit_2 (`KismetSystemLibrary.LineTraceSingle` :`Start` _returnvalue_3 :`End` (+ _returnvalue_3 (* (`KismetMathLibrary.RandomUnitVectorInConeInDegrees` (`local.RandomDirection`) (`self.SecondaryTraceDirectionRandomAngle`)) (`self.MaxRadius`))) :`TraceChannel` "TraceTypeQuery1" :`DrawTime` 1.0))
              (bind (_bblockinghit_2 _binitialoverlap_2 _time_2 _distance_2 _location_2 _impactpoint_2 _normal_2 _impactnormal_2) (`GameplayStatics.BreakHitResult` _outhit_2))
              (if _bblockinghit_2
                (bind _returnvalue_6 (`NiagaraFunctionLibrary.SpawnSystemAttached` "/Game/Production/Effects/Environment/LightningExplosion/NS_LightningArcs_Secondary.NS_LightningArcs_Secondary" (`self.DefaultSceneRoot`) "None" (0.0 0.0 0.0) (struct) "KeepRelativeOffset" true))
                (`NiagaraComponent.SetVariableVec3` _returnvalue_6 "BeamStartPoint" (`local.LasthitWithOffset`))
                (`NiagaraComponent.SetVariableVec3` _returnvalue_6 "BeamEndPoint" (+ _impactpoint_2 (* _impactnormal_2 (`local.ImpactOffset`))))
                (`NiagaraComponent.SetVariableVec3` _returnvalue_6 "ImpactNormal" _impactnormal_2)
                ;[1 1 1] UpdateLasthitInfo
                (set `local.LasthitLocation` _impactpoint_2)
                (set `local.LasthitWithOffset` _impactpoint_2)
                (set `local.LasthitNormal` _impactnormal_2)
                (else
                  (break))))))))))

(fn `UserConstructionScript`)