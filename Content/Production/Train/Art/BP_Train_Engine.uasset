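; BP_Train_Engine is a train engine actor that applies a shared material progress value to its static meshes.
; The construction script rebuilds StaticMeshElements from the static mesh components under Scene and passes each to SetMaterialInstanceProgress.
; That function stores MaterialProgress and writes it to custom primitive data slot 0, so no dynamic material instances are created.
; The event graph holds only disabled placeholder events.
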(fn `Set Material Instance Progress`
  (params (MaterialProgress :type "Float (double-precision)") (`Static Mesh` :type "StaticMeshComponent Object Reference"))
  (bind _output_get (set `self.Material Progress` MaterialProgress))
  (`PrimitiveComponent.SetCustomPrimitiveDataFloat` `Static Mesh` 0 _output_get))

(fn `UserConstructionScript`
  (bind _static_mesh_elements (`self.Static Mesh Elements`))
  (`KismetArrayLibrary.Array_Clear` _static_mesh_elements)
  (for _array_element (`SceneComponent.GetChildrenComponents` (`self.Scene`) true)
    (bind _asstatic_mesh_component (cast `StaticMeshComponent` _array_element))
    (`KismetArrayLibrary.Array_Add` _static_mesh_elements _asstatic_mesh_component)
    (`self.Set Material Instance Progress` (`self.Material Progress`) _asstatic_mesh_component)))